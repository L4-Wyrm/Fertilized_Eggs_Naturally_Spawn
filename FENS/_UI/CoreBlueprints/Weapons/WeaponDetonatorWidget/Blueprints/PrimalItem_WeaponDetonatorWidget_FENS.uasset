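; Primal item Blueprint for the FENS weapon detonator widget, handling localization of its displayed name and description.
; It overrides the item name and description getters, routing each through a helper that checks the two-letter ISO language code.
; When the code matches RU, the helpers return the stored Russian strings; otherwise they pass the incoming text through unchanged.
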(fn `BPCheckDescriptionLanguage`
  (params (InDescription :type String))
  (returns (ReturnValue :type String))
  (return (`KismetMathLibrary.SelectString` (`self.RU_DescriptionString`) InDescription (`KismetStringLibrary.MatchesWildcard` (`VictoryCore.GetTwoLetterISOLanguageName`) "RU"))))

(fn `BPCheckNameLanguage`
  (params (ItemNameIn :type String))
  (returns (ReturnValue :type String))
  (return (`KismetMathLibrary.SelectString` (`self.RU_ItemNameString`) ItemNameIn (`KismetStringLibrary.MatchesWildcard` (`VictoryCore.GetTwoLetterISOLanguageName`) "RU"))))

(fn `BPGetItemDescription`
  (params (InDescription :type String) (bGetLongDescription :type Boolean) (ForPC :type "ShooterPlayerController Object Reference"))
  (returns (ReturnValue :type String))
  (bind _returnvalue (`self.BPCheckDescriptionLanguage` InDescription))
  (return _returnvalue))

(fn `BPGetItemName`
  (params (ItemNameIn :type String) (ForPC :type "ShooterPlayerController Object Reference"))
  (returns (ReturnValue :type String))
  (bind _returnvalue (`self.BPCheckNameLanguage` ItemNameIn))
  (return _returnvalue))