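; Base FENS nest structure that turns nearby wild creatures hostile when a player damages or destroys it.
; BeginPlay optionally fires spawn FX and binds the damage handler, then applies delayed self-damage.
; Player damage and the timed destroy multi-use entry use octree searches to force-aggro configured creature classes onto local player characters.
; Names and menu text switch between Russian, English or custom strings, using INI options or a polling timer.
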(event `self.ReceiveBeginPlay`
  (bind _buseinioptions (`self.bUseINIOptions`))
  (`parent.ReceiveBeginPlay`)
  (`|ExecutionSequence`
    (:`then_0`
      (if (`self.bEnableNestSpawningFX`)
        (`ActorComponent.Activate` (`self.SpawnIn`) false)
        (`ActorComponent.Activate` (`self.NestSpawnFX1`) false)
        (`ActorComponent.Activate` (`self.NestSpawnFX2`) false)
        (`ActorComponent.Activate` (`self.SoundToPlay`) false)
        (add `self.OnTakeAnyDamage` (delegate `OnTakeAnyDamage_Event`))))
    (:`then_1`
      (`KismetSystemLibrary.Delay` (`self.DelayBeforeTakeDamage`))
      (`GameplayStatics.ApplyDamage` self 1000.0 null null "/Game/PrimalEarth/CoreBlueprints/DamageTypes/DmgType_Melee.DmgType_Melee_C"))
    (:`then_2`
      (if _buseinioptions
        (`self.INIOptions`)))
    (:`then_3`
      (if _buseinioptions
        (if (not (`self.bIsCustomLocalization`))
          (`self.BPCheckGameLanguage`)
          (else
            (`self.BPCheckGameCustomLanguage`)))))
    (:`then_4`
      (if (not _buseinioptions)
        (`KismetSystemLibrary.K2_SetTimer` null "Event_CheckForLocalizationValuesChange" 0.3 true)))))

(event `Event_CheckForLocalizationValuesChange`
  (if (not (`self.bIsCustomLocalization`))
    (`self.BPCheckGameLanguage`)
    (else
      (`self.BPCheckGameCustomLanguage`))))

(event `OnTakeAnyDamage_Event` :!signature `self.OnTakeAnyDamage`
  (params (Damage :type "Float (double-precision)") (DamageType :type "DamageType Object Reference") (InstigatedBy :type "Controller Object Reference") (DamageCauser :type "Actor Object Reference"))
  (bind _returnvalue (`self.K2_GetActorLocation`))
  (bind _returnvalue_2 (`VictoryCore.GetAllLocalPlayerCharacters`))
  (bind _returnvalue_3 (`self.K2_GetWorld`))
  (bind _flwildcreatureaggroradius (`self.flWildCreatureAggroRadius`))
  (cast `ShooterPlayerController` InstigatedBy)
  (if (not (`self.bUseListOfWildCreatures`))
    (bind _returnvalue_4 (`VictoryCore.ServerOctreeOverlapActorsClass` _returnvalue_3 _returnvalue _flwildcreatureaggroradius "DINOPAWNS" (`self.WildCreatureToAggro`)))
    (for _array_element _returnvalue_4
      (bind _asprimaldinocharacter (cast `PrimalDinoCharacter` _array_element))
      (`/Engine/EditorBlueprintResources/StandardMacros.IsValid` _asprimaldinocharacter
        (:`Is Valid`
          (for _array_element_2 _returnvalue_2
            (bind _asshootercharacter (cast `ShooterCharacter` _array_element_2))
            (`PrimalDinoCharacter.BPSetForcedAggro` _asprimaldinocharacter _asshootercharacter 999.9 999.9)))))
    (else
      (for _array_element_3 (`self.WildCreaturesToAggroList`)
        (bind _returnvalue_5 (`VictoryCore.ServerOctreeOverlapActorsClass` _returnvalue_3 _returnvalue _flwildcreatureaggroradius "DINOPAWNS" _array_element_3))
        (for _array_element_4 _returnvalue_5
          (bind _asprimaldinocharacter_2 (cast `PrimalDinoCharacter` _array_element_4))
          (`/Engine/EditorBlueprintResources/StandardMacros.IsValid` _asprimaldinocharacter_2
            (:`Is Valid`
              (for _array_element_5 _returnvalue_2
                (bind _asshootercharacter_2 (cast `ShooterCharacter` _array_element_5))
                (`PrimalDinoCharacter.BPSetForcedAggro` _asprimaldinocharacter_2 _asshootercharacter_2 999.9 999.9)))))))))

(fn `BPCheckGameCustomLanguage`
  (set `self.DescriptiveName` (`self.DescriptiveNameStringCustom`))
  (set `self.DestroyNestString` (`self.DestroyNestStringCustom`))
  (set `self.NestOptionsString` (`self.NestOptionsStringCustom`)))

(fn `BPCheckGameLanguage`
  (bind _returnvalue (`VictoryCore.GetTwoLetterISOLanguageName`))
  (set `self.DescriptiveName` (`KismetMathLibrary.SelectString` (`self.DescriptiveNameStringRU`) (`self.DescriptiveNameStringEN`) (`KismetStringLibrary.MatchesWildcard` _returnvalue "RU")))
  (set `self.NestOptionsString` (`KismetMathLibrary.SelectString` (`self.NestOptionsStringRU`) (`self.NestOptionsStringEN`) (`KismetStringLibrary.MatchesWildcard` _returnvalue "RU")))
  (set `self.DestroyNestString` (`KismetMathLibrary.SelectString` (`self.DestroyNestStringRU`) (`self.DestroyNestStringEN`) (`KismetStringLibrary.MatchesWildcard` _returnvalue "RU"))))

(fn `BPGetMultiUseEntries`
  (params (ForPC :type "PlayerController Object Reference") (MultiUseEntries :type "Array of Actor.MultiUseEntry Structure (by ref)"))
  (returns (ReturnValue :type "Array of Actor.MultiUseEntry Structure"))
  (`KismetArrayLibrary.Array_Add` MultiUseEntries (make `Actor.MultiUseEntry` null (`self.NestOptionsString`) 10010 4 true))
  (`KismetArrayLibrary.Array_Append` MultiUseEntries (`|MakeArray` (make `Actor.MultiUseEntry` null (`self.DestroyNestString`) 10011 1 false false false false false false false false false false false false false false 0 (struct :`B` 175 :`G` 175 :`R` 175 :`A` 255) (struct :`B` 255 :`G` 255 :`R` 255 :`A` 255) 0.0 3.0 (`self.DestroySound`))))
  (return MultiUseEntries))

(fn `BPTryMultiUse`
  (params (ForPC :type "PlayerController Object Reference") (UseIndex :type Integer))
  (returns (ReturnValue :type Boolean))
  (switch `int` UseIndex
    (:`Default`
      (return true))
    (:`10011`
      (`GameplayStatics.ApplyDamage` self 9999.9 null (`self.Instigator`))
      (bind _returnvalue (`VictoryCore.ServerOctreeOverlapActorsClass` (`self.K2_GetWorld`) (0.0 0.0 0.0) (`self.flWildCreatureAggroRadius`) "DINOPAWNS" (`self.WildCreatureToAggro`)))
      (for _array_element _returnvalue
        (bind _asprimaldinocharacter (cast `PrimalDinoCharacter` _array_element))
        (`/Engine/EditorBlueprintResources/StandardMacros.IsValid` _asprimaldinocharacter
          (:`Is Valid`
            (for _array_element_2 (`VictoryCore.GetAllLocalPlayerCharacters`)
              (bind _asshootercharacter (cast `ShooterCharacter` _array_element_2))
              (`PrimalDinoCharacter.BPSetForcedAggro` _asprimaldinocharacter _asshootercharacter 999.9 999.9))))))))

(fn `INIOptions`
  (`/Engine/EditorBlueprintResources/ActorMacros.Switch Has Authority`
    (:`Authority`
      (bind _asshootergamemode (cast `ShooterGameMode` (`GameplayStatics.GetGameMode`)))
      (if (`self.bIsCustomLocalization`)
        (`|ExecutionSequence`
          (:`then_0`
            (`ShooterGameMode.InitOptionString` _asshootergamemode "" "FENS_CustomLocalization" (`self.NestOptionsStringCustom`))
            (`ShooterGameMode.InitOptionString` _asshootergamemode "" "FENS_CustomLocalization" (`self.DestroyNestStringCustom`))
            (`ShooterGameMode.InitOptionString` _asshootergamemode "" "FENS_CustomLocalization" (`self.DescriptiveNameStringCustom`)))
          (:`then_1`
            (bind _returnvalue (`ShooterGameMode.GetStringOption` _asshootergamemode "FENS_CustomLocalization" (`self.NestOptionsStringCustom`)))
            (set `self.NestOptionsStringCustom` _returnvalue)
            (bind _returnvalue_2 (`ShooterGameMode.GetStringOption` _asshootergamemode "FENS_CustomLocalization" (`self.DestroyNestStringCustom`)))
            (set `self.DestroyNestStringCustom` _returnvalue_2)
            (bind _returnvalue_3 (`ShooterGameMode.GetStringOption` _asshootergamemode "FENS_CustomLocalization" (`self.DescriptiveNameStringCustom`)))
            (set `self.DescriptiveNameStringCustom` _returnvalue_3)))))))

(fn `UserConstructionScript`)