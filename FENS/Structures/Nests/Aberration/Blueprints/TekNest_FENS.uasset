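; Tek variant of the FENS nest structure that adds its own spawn-in particle and a choice of Tek materials.
; On BeginPlay the authority reads a FENSSettings INI option choosing between newer ripple materials and older ones, applied to both mesh slots after a delay.
; Delayed steps also activate the Tek particle and touch the parent's SpawnIn, which DisableParentSpawnInParticle sets to not hidden despite its name.
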(event `self.ReceiveBeginPlay`
  (`parent.ReceiveBeginPlay`)
  (`|ExecutionSequence`
    (:`then_0`
      (`KismetSystemLibrary.Delay` 4.0)
      (`self.SetNewestTekNestMaterial`))
    (:`then_1`
      (`self.INIOptions`))
    (:`then_2`
      (`KismetSystemLibrary.Delay` 3.0)
      (`self.EnableParticle`))
    (:`then_3`
      (`KismetSystemLibrary.Delay` 0.3)
      (`self.DisableParentSpawnInParticle`))))

(fn `DisableParentSpawnInParticle`
  (bind _asnest_fens_c (cast `/Game/Mods/FENS/Structures/Nests/PrimalEarth/Blueprints/BaseBPs/Nest_FENS` self))
  (`SceneComponent.SetHiddenInGame` (`/Game/Mods/FENS/Structures/Nests/PrimalEarth/Blueprints/BaseBPs/Nest_FENS.SpawnIn` _asnest_fens_c) false false))

(fn `EnableParticle`
  (bind _asteknest_fens_c (cast `/FENS/Structures/Nests/Aberration/Blueprints/TekNest_FENS` self))
  (`ActorComponent.Activate` (`/FENS/Structures/Nests/Aberration/Blueprints/TekNest_FENS.SpawnInTek` _asteknest_fens_c) false))

(fn `INIOptions`
  (`/Engine/EditorBlueprintResources/ActorMacros.Switch Has Authority`
    (:`Authority`
      (bind _asshootergamemode (cast `ShooterGameMode` (`GameplayStatics.GetGameMode`)))
      (`|ExecutionSequence`
        (:`then_0`
          (`ShooterGameMode.InitOptionBool` _asshootergamemode "" (`self.FENS_Settings`) (`self.UseNewestNestTekMaterial`) (`self.bUseNewestTekNestMaterial`)))
        (:`then_1`
          (bind _returnvalue (`ShooterGameMode.GetBoolOptionIni` _asshootergamemode (`self.FENS_Settings`) (`self.UseNewestNestTekMaterial`) true))
          (set `self.bUseNewestTekNestMaterial` _returnvalue))))))

(fn `SetNewestTekNestMaterial`
  (bind _mystaticmesh (`self.MyStaticMesh`))
  (if (`self.bUseNewestTekNestMaterial`)
    (`|ExecutionSequence`
      (:`then_0`
        (`PrimitiveComponent.SetMaterial` _mystaticmesh 0 "/Game/Mods/FENS/EndGame/Test/TekNest/MIC_TekNestRipple_FENS.MIC_TekNestRipple_FENS"))
      (:`then_1`
        (`PrimitiveComponent.SetMaterial` _mystaticmesh 1 "/Game/Mods/FENS/EndGame/Test/TekNest/MIC_TekNestSkullFeamerRipple_FENS.MIC_TekNestSkullFeamerRipple_FENS")))
    (else
      (`|ExecutionSequence`
        (:`then_0`
          (`PrimitiveComponent.SetMaterial` _mystaticmesh 0 "/Game/Aberration/Environment/DrakeTrench/Materials/Nest2_MIC.Nest2_MIC"))
        (:`then_1`
          (`PrimitiveComponent.SetMaterial` _mystaticmesh 1 "/Game/ScorchedEarth/Environment/Shared/catacomb/MI_SkullFeamer2.MI_SkullFeamer2"))))))

(fn `UserConstructionScript`
  (`parent.UserConstructionScript`))