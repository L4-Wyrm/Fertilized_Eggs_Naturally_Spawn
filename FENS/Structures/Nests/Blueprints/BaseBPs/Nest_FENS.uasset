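; Base nest structure Blueprint for FENS that plays a spawn-in effect and automatically destroys itself with heavy melee damage after a delay.
; On BeginPlay it applies the spawn-in material, then after one second switches to the spawn-out material and activates the SpawnIn component.
; The authority reads the delay from the FENS_Settings INI via ShooterGameMode, but only after the self-damage timer has started with the existing value.
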(event `self.ReceiveBeginPlay`
  (bind _mystaticmesh (`self.MyStaticMesh`))
  (bind _mystaticmesh_2 (`self.MyStaticMesh`))
  (`parent.ReceiveBeginPlay`)
  (`|ExecutionSequence`
    (:`then_0`
      (`PrimitiveComponent.SetMaterial` _mystaticmesh_2 0 (`self.SpawnInMaterial`))
      (`KismetSystemLibrary.Delay` 1.0 :!label _label)
      (`|ExecutionSequence`
        (:`then_0`
          (`PrimitiveComponent.SetMaterial` _mystaticmesh 0 (`self.SpawnOutMaterial`)))
        (:`then_1`
          (`PrimitiveComponent.SetMaterial` _mystaticmesh 1 (`self.SpawnOutMaterial`))))
      (bind _asnest_fens_c (cast `/FENS/Structures/Nests/Blueprints/BaseBPs/Nest_FENS` self))
      (`ActorComponent.Activate` (`/FENS/Structures/Nests/Blueprints/BaseBPs/Nest_FENS.SpawnIn` _asnest_fens_c) false))
    (:`then_1`
      (`PrimitiveComponent.SetMaterial` _mystaticmesh_2 1 (`self.SpawnInMaterial`))
      (goto _label))
    (:`then_2`
      (`KismetSystemLibrary.Delay` (`self.DelayBeforeTakeDamage`))
      (`GameplayStatics.ApplyDamage` self 1000.0 null null "/Game/PrimalEarth/CoreBlueprints/DamageTypes/DmgType_Melee.DmgType_Melee_C"))
    (:`then_3`
      (`self.INIOptions`))))

(fn `INIOptions`
  (`/Engine/EditorBlueprintResources/ActorMacros.Switch Has Authority`
    (:`Authority`
      (bind _asshootergamemode (cast `ShooterGameMode` (`GameplayStatics.GetGameMode`)))
      (`|ExecutionSequence`
        (:`then_0`
          (`ShooterGameMode.InitOptionFloat` _asshootergamemode "" "FENS_Settings" "DelayBeforeAutoDelete" (`self.DelayBeforeTakeDamage`)))
        (:`then_1`
          (bind _returnvalue (`ShooterGameMode.GetFloatOptionIni` _asshootergamemode "FENS_Settings" "DelayBeforeAutoDelete"))
          (set `self.DelayBeforeTakeDamage` _returnvalue))))))

(fn `UserConstructionScript`)