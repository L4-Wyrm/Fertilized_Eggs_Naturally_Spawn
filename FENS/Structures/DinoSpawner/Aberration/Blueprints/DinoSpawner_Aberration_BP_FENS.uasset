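; Aberration variant of the FENS DinoSpawner structure, handling the pedestal egg, core and antenna particle effects.
; On BeginPlay, preview placements switch off the egg effect, while placed structures turn it on, then enable or disable all effects per IsSmokeEffectsEnabled.
; On authority, INIOptions then registers and reads that flag through ShooterGameMode's INI options, after the effects have already been set.
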(event `self.ReceiveBeginPlay`
  (bind _pedestaleggfx (`self.PedestalEggFX`))
  (if (`self.bIsPreviewStructure`)
    (`ActorComponent.Deactivate` _pedestaleggfx)
    (else
      (`ActorComponent.Activate` _pedestaleggfx false)
      (`|ExecutionSequence`
        (:`then_0`
          (if (`self.bIsSmokeEffectsEnabled`)
            (`self.SmokeEffectsEnable`)
            (else
              (`self.SmokeEffectsDisable`))))
        (:`then_1`
          (`self.INIOptions`))))))

(fn `INIOptions`
  (`/Engine/EditorBlueprintResources/ActorMacros.Switch Has Authority`
    (:`Authority`
      (bind _asshootergamemode (cast `ShooterGameMode` (`GameplayStatics.GetGameMode`)))
      (`|ExecutionSequence`
        (:`then_0`
          (`ShooterGameMode.InitOptionBool` _asshootergamemode "" (`self.SpawnerHeader`) (`self.IsSmokeEffectsEnabled`) (`self.bIsSmokeEffectsEnabled`)))
        (:`then_1`
          (bind _returnvalue (`ShooterGameMode.GetBoolOptionIni` _asshootergamemode (`self.SpawnerHeader`) (`self.IsSmokeEffectsEnabled`) false))
          (set `self.bIsSmokeEffectsEnabled` _returnvalue))))))

(fn `SmokeEffectsDisable`
  (`ActorComponent.Deactivate` (`self.EggPedestalCoreFX`))
  (`ActorComponent.Deactivate` (`self.EggPedestalAntennaFX1`))
  (`ActorComponent.Deactivate` (`self.EggPedestalAntennaFX2`))
  (`ActorComponent.Deactivate` (`self.EggPedestalAntennaFX3`))
  (`ActorComponent.Deactivate` (`self.EggPedestalAntennaFX4`))
  (`ActorComponent.Deactivate` (`self.EggPedestalAntennaFX5`))
  (`ActorComponent.Deactivate` (`self.EggPedestalAntennaFX6`))
  (`ActorComponent.Deactivate` (`self.EggPedestalAntennaFX7`))
  (`ActorComponent.Deactivate` (`self.EggPedestalAntennaFX8`))
  (`ActorComponent.Deactivate` (`self.PedestalEggFX`)))

(fn `SmokeEffectsEnable`
  (`ActorComponent.Activate` (`self.EggPedestalAntennaFX6`) false)
  (`ActorComponent.Activate` (`self.EggPedestalAntennaFX7`) false)
  (`ActorComponent.Activate` (`self.EggPedestalAntennaFX8`) false)
  (`ActorComponent.Activate` (`self.PedestalEggFX`) false)
  (`ActorComponent.Activate` (`self.EggPedestalAntennaFX5`) false)
  (`ActorComponent.Activate` (`self.EggPedestalAntennaFX4`) false)
  (`ActorComponent.Activate` (`self.EggPedestalAntennaFX3`) false)
  (`ActorComponent.Activate` (`self.EggPedestalAntennaFX2`) false)
  (`ActorComponent.Activate` (`self.EggPedestalAntennaFX1`) false)
  (`ActorComponent.Activate` (`self.EggPedestalCoreFX`) false))

(fn `UserConstructionScript`
  (`parent.UserConstructionScript`))