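; Test dino spawner Blueprint whose only logic here destroys test dinosaur characters that touch it; no spawning happens in this graph.
; On DinoCollisionSphere begin overlap, a Sequence casts the other actor to each of six classes: the base test dino plus Allo, Dilo, Raptor, corrupt Raptor and Spindles test-map characters.
; The base dino has its own DestroyActor call, while the other five casts share one multi-target DestroyActor node.
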(event `self.DinoCollisionSphere.OnComponentBeginOverlap`
  (params (OtherActor :type "Actor Object Reference") (OtherComp :type "PrimitiveComponent Object Reference") (OtherBodyIndex :type Integer) (bFromSweep :type Boolean) (SweepResult :type "EngineTypes.HitResult Structure (by ref)"))
  (`|ExecutionSequence`
    (:`then_0`
      (bind _asdino_character_test_bp_fens_c (cast `/Game/Mods/FENS/CoreBlueprints/Dino_Character_Test_BP_FENS` OtherActor))
      (`self.K2_DestroyActor` _asdino_character_test_bp_fens_c))
    (:`then_1`
      (bind _asallotestmap_character_bp_fens_c (cast `/Game/Mods/FENS/Dinos/Allosaurus/AlloTestMap_Character_BP_FENS` OtherActor))
      (`self.K2_DestroyActor` (stale _asdilotestmap_character_bp_fens_c) :!label _label)
      (`self.K2_DestroyActor` _asallotestmap_character_bp_fens_c)
      (`self.K2_DestroyActor` (stale _asraptortestmap_character_bp_fens_c))
      (`self.K2_DestroyActor` (stale _asraptortestmap_character_bp_corrupt_fens_c))
      (`self.K2_DestroyActor` (stale _asspindlestestmap_character_bp_fens_c)))
    (:`then_2`
      (bind _asdilotestmap_character_bp_fens_c (cast `/Game/Mods/FENS/Dinos/Dilo/DiloTestMap_Character_BP_FENS` OtherActor))
      (goto _label))
    (:`then_3`
      (bind _asraptortestmap_character_bp_fens_c (cast `/Game/Mods/FENS/Dinos/Raptor/RaptorTestMap_Character_BP_FENS` OtherActor))
      (goto _label))
    (:`then_4`
      (bind _asraptortestmap_character_bp_corrupt_fens_c (cast `/Game/Mods/FENS/Extinction/Dinos/Corrupt/Raptor/RaptorTestMap_Character_BP_Corrupt_FENS` OtherActor))
      (goto _label))
    (:`then_5`
      (bind _asspindlestestmap_character_bp_fens_c (cast `/Game/Mods/FENS/Extinction/Dinos/Spindles/SpindlesTestMap_Character_BP_FENS` OtherActor))
      (goto _label))))

(fn `UserConstructionScript`
  (`parent.UserConstructionScript`))