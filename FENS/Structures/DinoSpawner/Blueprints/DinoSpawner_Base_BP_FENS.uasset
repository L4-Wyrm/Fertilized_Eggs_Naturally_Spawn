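; Base dino spawner structure that periodically spawns random creatures from CreaturesArray near itself, skipped for placement previews.
; A looping timer runs RandomiseDino, with SpawningChance serving as both the interval and the roll threshold, and spawns at random radius-based offsets above the structure.
; Any Dino_Character_BP_FENS entering Sphere1 is destroyed.
; INIOptions, not called within this graph, reads chance and radius settings from ShooterGameMode INI on authority.
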(event `self.ReceiveBeginPlay`
  (if (not (`self.bIsPreviewStructure`))
    (`|ExecutionSequence`
      (:`then_0`
        (`KismetSystemLibrary.K2_SetTimer` null "RandomiseDino" (`self.SpawningChance`) true)))))

(event `self.Sphere1.OnComponentBeginOverlap`
  (params (OtherActor :type "Actor Object Reference") (OtherComp :type "PrimitiveComponent Object Reference") (OtherBodyIndex :type Integer) (bFromSweep :type Boolean) (SweepResult :type "EngineTypes.HitResult Structure (by ref)"))
  (bind _asdino_character_bp_fens_c (cast `/Game/Mods/FENS/CoreBlueprints/Dino_Character_BP_FENS` OtherActor))
  (`self.K2_DestroyActor` _asdino_character_bp_fens_c))

(fn `INIOptions`
  (`/Engine/EditorBlueprintResources/ActorMacros.Switch Has Authority`
    (:`Authority`
      (bind _asshootergamemode (cast `ShooterGameMode` (`GameplayStatics.GetGameMode`)))
      (bind _returnvalue (`ShooterGameMode.GetFloatOptionIni` _asshootergamemode (`self.FENSSpawnerTitle`) (`self.SpawningChanceString`)))
      (set `self.SpawningChance` _returnvalue)
      (`ShooterGameMode.InitOptionFloat` _asshootergamemode "" (`self.FENSSpawnerTitle`) (`self.SpawningChanceString`) (`self.SpawningChance`))
      (bind _returnvalue_2 (`ShooterGameMode.GetFloatOptionIni` _asshootergamemode (`self.FENSSpawnerTitle`) (`self.MaxRadiusString`)))
      (set `self.MaxRadius` _returnvalue_2)
      (`ShooterGameMode.InitOptionFloat` _asshootergamemode "" (`self.FENSSpawnerTitle`) (`self.MaxRadiusString`) (`self.MaxRadius`))
      (bind _returnvalue_3 (`ShooterGameMode.GetFloatOptionIni` _asshootergamemode (`self.FENSSpawnerTitle`) (`self.MinRadiusString`)))
      (set `self.MinRadius` _returnvalue_3)
      (`ShooterGameMode.InitOptionFloat` _asshootergamemode "" (`self.FENSSpawnerTitle`) (`self.MinRadiusString`) (`self.MinRadius`)))))

(fn `RandomiseDino`
  (bind _creaturesarray (`self.CreaturesArray`))
  (bind _returnvalue (`KismetMathLibrary.RandomFloatInRange` (`self.MinRadius`) (`self.MaxRadius`)))
  (if (<= (`KismetMathLibrary.RandomFloat`) (`self.SpawningChance`))
    (`KismetArrayLibrary.Array_Shuffle` _creaturesarray)
    (`|SpawnActorFromClass` (`KismetArrayLibrary.Array_Get` _creaturesarray (`KismetMathLibrary.RandomIntegerInRange` 0 (`KismetArrayLibrary.Array_LastIndex` (`self.CreaturesArray`)))) (`KismetMathLibrary.MakeTransform` (`KismetMathLibrary.MakeVector` (+ (.x (.location (`self.GetTransform` self))) _returnvalue) (+ (.y (.location (`self.GetTransform` self))) _returnvalue) (+ (.z (.location (`self.GetTransform` self))) (`KismetMathLibrary.RandomFloatInRange` 300.0 450.0))) (.rotation (`self.GetTransform` self)) (.scale (`self.GetTransform` self))) true)))

(fn `UserConstructionScript`
  (`parent.UserConstructionScript`))