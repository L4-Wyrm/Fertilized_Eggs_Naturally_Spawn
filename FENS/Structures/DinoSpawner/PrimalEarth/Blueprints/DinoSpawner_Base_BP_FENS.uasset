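; Base dino spawner structure that, when not a preview, periodically spawns random creatures at positive X/Y offsets from itself.
; A looping timer, set before INI options load, rolls vanilla or marine spawns; successful vanilla spawns also roll unique and optional bionic ones.
; Server INI options supply chances, radii and delay.
; A min-radius sphere destroys overlapping FENS dinos; failed bionic, marine and unique rolls call destroy on spawnActor.
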(event `self.ReceiveBeginPlay`
  (if (not (`self.bIsPreviewStructure`))
    (`|ExecutionSequence`
      (:`then_0`
        (`KismetSystemLibrary.K2_SetTimer` null "EventInitSpawn" (`self.DelayBeforeSpawn`) true))
      (:`then_1`
        (`self.INIOptions`))
      (:`then_2`
        (`self.SetSphereRadius`)))))

(event `self.EggSpawnCollision.OnComponentBeginOverlap`
  (params (OtherActor :type "Actor Object Reference") (OtherComp :type "PrimitiveComponent Object Reference") (OtherBodyIndex :type Integer) (bFromSweep :type Boolean) (SweepResult :type "EngineTypes.HitResult Structure (by ref)"))
  (bind _asdino_character_bp_fens_c (cast `/Game/Mods/FENS/CoreBlueprints/Dino_Character_BP_FENS` OtherActor))
  (`self.K2_DestroyActor` _asdino_character_bp_fens_c))

(event `EventInitSpawn`
  (`|ExecutionSequence`
    (:`then_0`
      (if (`self.bIsVanillaSpawner`)
        (`self.SpawnRandomisedDino`)))
    (:`then_1`
      (if (`self.bIsMarineSpawner`)
        (`self.SpawnRandomisedMarineDino`)))))

(fn `INIOptions`
  (`/Engine/EditorBlueprintResources/ActorMacros.Switch Has Authority`
    (:`Authority`
      (bind _asshootergamemode (cast `ShooterGameMode` (`GameplayStatics.GetGameMode`)))
      (`|ExecutionSequence`
        (:`then_0`
          (`ShooterGameMode.InitOptionFloat` _asshootergamemode "" (`self.FENSSpawnerTitle`) (`self.SpawningChanceString`) (`self.SpawningChance`))
          (`ShooterGameMode.InitOptionFloat` _asshootergamemode "" (`self.FENSSpawnerTitle`) (`self.MinSpawnRadiusString`) (`self.CollisionSphereMinRadius`))
          (`ShooterGameMode.InitOptionFloat` _asshootergamemode "" (`self.FENSSpawnerTitle`) (`self.DelayBeforeSpawnString`) (`self.DelayBeforeSpawn`))
          (`ShooterGameMode.InitOptionFloat` _asshootergamemode "" (`self.FENSSpawnerTitle`) (`self.SpawningChanceBionicString`) (`self.SpawningChanceBionic`))
          (`ShooterGameMode.InitOptionFloat` _asshootergamemode "" (`self.FENSSpawnerTitle`) (`self.SpawningChanceUniqueString`) (`self.SpawningChanceUnique`))
          (`ShooterGameMode.InitOptionFloat` _asshootergamemode "" (`self.FENSSpawnerTitle`) (`self.MaxSpawnRadiusString`) (`self.CollisionSphereMaxRadius`)))
        (:`then_1`
          (bind _returnvalue (`ShooterGameMode.GetFloatOptionIni` _asshootergamemode (`self.FENSSpawnerTitle`) (`self.SpawningChanceString`)))
          (set `self.SpawningChance` _returnvalue)
          (bind _returnvalue_2 (`ShooterGameMode.GetFloatOptionIni` _asshootergamemode (`self.FENSSpawnerTitle`) (`self.MinSpawnRadiusString`)))
          (set `self.CollisionSphereMinRadius` _returnvalue_2)
          (bind _returnvalue_3 (`ShooterGameMode.GetFloatOptionIni` _asshootergamemode (`self.FENSSpawnerTitle`) (`self.DelayBeforeSpawnString`)))
          (set `self.DelayBeforeSpawn` _returnvalue_3)
          (bind _returnvalue_4 (`ShooterGameMode.GetFloatOptionIni` _asshootergamemode (`self.FENSSpawnerTitle`) (`self.SpawningChanceBionicString`)))
          (set `self.SpawningChanceBionic` _returnvalue_4)
          (bind _returnvalue_5 (`ShooterGameMode.GetFloatOptionIni` _asshootergamemode (`self.FENSSpawnerTitle`) (`self.SpawningChanceUniqueString`)))
          (set `self.SpawningChanceUnique` _returnvalue_5)
          (bind _returnvalue_6 (`ShooterGameMode.GetFloatOptionIni` _asshootergamemode (`self.FENSSpawnerTitle`) (`self.MaxSpawnRadiusString`)))
          (set `self.CollisionSphereMaxRadius` _returnvalue_6))))))

(fn `SetSphereRadius`
  (`SphereComponent.SetSphereRadius` (`self.EggSpawnCollision`) (`self.CollisionSphereMinRadius`) true))

(fn `SpawnRandomisedBionicDino`
  (bind _collisionsphereminradius (`self.CollisionSphereMinRadius`))
  (bind _collisionsphereminradius_2 (`self.CollisionSphereMinRadius`))
  (bind _bioniccreaturelist (`self.BionicCreatureList`))
  (if (<= (`KismetMathLibrary.RandomFloat`) (`self.SpawningChanceBionic`))
    (`KismetArrayLibrary.Array_Shuffle` _bioniccreaturelist)
    (bind _returnvalue (`|SpawnActorFromClass` (`KismetArrayLibrary.Array_Get` _bioniccreaturelist (`KismetMathLibrary.RandomIntegerInRange` 0 (`KismetArrayLibrary.Array_LastIndex` (`self.BionicCreatureList`)))) (`KismetMathLibrary.MakeTransform` (`KismetMathLibrary.MakeVector` (+ (.x (.location (`KismetMathLibrary.Conv_VectorToTransform` (`self.K2_GetActorLocation` self)))) (`KismetMathLibrary.RandomFloatInRange` _collisionsphereminradius_2 (+ _collisionsphereminradius_2 (`self.CollisionSphereMaxRadius`)))) (+ (.y (.location (`KismetMathLibrary.Conv_VectorToTransform` (`self.K2_GetActorLocation` self)))) (`KismetMathLibrary.RandomFloatInRange` _collisionsphereminradius (+ _collisionsphereminradius (`self.CollisionSphereMaxRadius`)))) (+ (.z (.location (`KismetMathLibrary.Conv_VectorToTransform` (`self.K2_GetActorLocation` self)))) 150.0)) (.rotation (`KismetMathLibrary.Conv_VectorToTransform` (`self.K2_GetActorLocation` self))) (.scale (`KismetMathLibrary.Conv_VectorToTransform` (`self.K2_GetActorLocation` self)))) true))
    (if (not (`VictoryCore.IsShipping`))
      (if (`VictoryCore.IsPlayInEditor`)
        (bind _asprimaldinocharacter (cast `PrimalDinoCharacter` _returnvalue))
        (`PrimalDinoCharacter.BPUnstasis` _asprimaldinocharacter)))
    (else
      (`self.K2_DestroyActor` _returnvalue))))

(fn `SpawnRandomisedDino`
  (bind _collisionsphereminradius (`self.CollisionSphereMinRadius`))
  (bind _collisionsphereminradius_2 (`self.CollisionSphereMinRadius`))
  (bind _creaturelist (`self.CreatureList`))
  (if (<= (`KismetMathLibrary.RandomFloat`) (`self.SpawningChance`))
    (`KismetArrayLibrary.Array_Shuffle` _creaturelist)
    (bind _returnvalue (`|SpawnActorFromClass` (`KismetArrayLibrary.Array_Get` _creaturelist (`KismetMathLibrary.RandomIntegerInRange` 0 (`KismetArrayLibrary.Array_LastIndex` (`self.CreatureList`)))) (`KismetMathLibrary.MakeTransform` (`KismetMathLibrary.MakeVector` (+ (.x (.location (`KismetMathLibrary.Conv_VectorToTransform` (`self.K2_GetActorLocation` self)))) (`KismetMathLibrary.RandomFloatInRange` _collisionsphereminradius_2 (+ _collisionsphereminradius_2 (`self.CollisionSphereMaxRadius`)))) (+ (.y (.location (`KismetMathLibrary.Conv_VectorToTransform` (`self.K2_GetActorLocation` self)))) (`KismetMathLibrary.RandomFloatInRange` _collisionsphereminradius (+ _collisionsphereminradius (`self.CollisionSphereMaxRadius`)))) (+ (.z (.location (`KismetMathLibrary.Conv_VectorToTransform` (`self.K2_GetActorLocation` self)))) 150.0)) (.rotation (`KismetMathLibrary.Conv_VectorToTransform` (`self.K2_GetActorLocation` self))) (.scale (`KismetMathLibrary.Conv_VectorToTransform` (`self.K2_GetActorLocation` self)))) true))
    (`|ExecutionSequence`
      (:`then_0`
        (if (not (`VictoryCore.IsShipping`))
          (if (`VictoryCore.IsPlayInEditor`)
            (bind _asprimaldinocharacter (cast `PrimalDinoCharacter` _returnvalue))
            (`PrimalDinoCharacter.BPUnstasis` _asprimaldinocharacter))))
      (:`then_1`
        (if (`self.bIsBionicSpawner`)
          (`self.SpawnRandomisedBionicDino`)))
      (:`then_2`
        (`self.SpawnRandomisedUniqueDino`)))))

(fn `SpawnRandomisedMarineDino`
  (bind _collisionsphereminradius (`self.CollisionSphereMinRadius`))
  (bind _collisionsphereminradius_2 (`self.CollisionSphereMinRadius`))
  (bind _marinecreaturelist (`self.MarineCreatureList`))
  (if (<= (`KismetMathLibrary.RandomFloat`) (`self.SpawningChance`))
    (`KismetArrayLibrary.Array_Shuffle` _marinecreaturelist)
    (bind _returnvalue (`|SpawnActorFromClass` (`KismetArrayLibrary.Array_Get` _marinecreaturelist (`KismetMathLibrary.RandomIntegerInRange` 0 (`KismetArrayLibrary.Array_LastIndex` (`self.MarineCreatureList`)))) (`KismetMathLibrary.MakeTransform` (`KismetMathLibrary.MakeVector` (+ (.x (.location (`KismetMathLibrary.Conv_VectorToTransform` (`self.K2_GetActorLocation` self)))) (`KismetMathLibrary.RandomFloatInRange` _collisionsphereminradius_2 (+ _collisionsphereminradius_2 (`self.CollisionSphereMaxRadius`)))) (+ (.y (.location (`KismetMathLibrary.Conv_VectorToTransform` (`self.K2_GetActorLocation` self)))) (`KismetMathLibrary.RandomFloatInRange` _collisionsphereminradius (+ _collisionsphereminradius (`self.CollisionSphereMaxRadius`)))) (+ (.z (.location (`KismetMathLibrary.Conv_VectorToTransform` (`self.K2_GetActorLocation` self)))) 150.0)) (.rotation (`KismetMathLibrary.Conv_VectorToTransform` (`self.K2_GetActorLocation` self))) (.scale (`KismetMathLibrary.Conv_VectorToTransform` (`self.K2_GetActorLocation` self)))) true))
    (if (not (`VictoryCore.IsShipping`))
      (if (`VictoryCore.IsPlayInEditor`)
        (bind _asprimaldinocharacter (cast `PrimalDinoCharacter` _returnvalue))
        (`PrimalDinoCharacter.BPUnstasis` _asprimaldinocharacter)))
    (else
      (`self.K2_DestroyActor` _returnvalue))))

(fn `SpawnRandomisedUniqueDino`
  (bind _collisionsphereminradius (`self.CollisionSphereMinRadius`))
  (bind _collisionsphereminradius_2 (`self.CollisionSphereMinRadius`))
  (bind _uniquecreaturelist (`self.UniqueCreatureList`))
  (if (<= (`KismetMathLibrary.RandomFloat`) (`self.SpawningChanceUnique`))
    (`KismetArrayLibrary.Array_Shuffle` _uniquecreaturelist)
    (bind _returnvalue (`|SpawnActorFromClass` (`KismetArrayLibrary.Array_Get` _uniquecreaturelist (`KismetMathLibrary.RandomIntegerInRange` 0 (`KismetArrayLibrary.Array_LastIndex` (`self.UniqueCreatureList`)))) (`KismetMathLibrary.MakeTransform` (`KismetMathLibrary.MakeVector` (+ (.x (.location (`KismetMathLibrary.Conv_VectorToTransform` (`self.K2_GetActorLocation` self)))) (`KismetMathLibrary.RandomFloatInRange` _collisionsphereminradius_2 (+ _collisionsphereminradius_2 (`self.CollisionSphereMaxRadius`)))) (+ (.y (.location (`KismetMathLibrary.Conv_VectorToTransform` (`self.K2_GetActorLocation` self)))) (`KismetMathLibrary.RandomFloatInRange` _collisionsphereminradius (+ _collisionsphereminradius (`self.CollisionSphereMaxRadius`)))) (+ (.z (.location (`KismetMathLibrary.Conv_VectorToTransform` (`self.K2_GetActorLocation` self)))) 150.0)) (.rotation (`KismetMathLibrary.Conv_VectorToTransform` (`self.K2_GetActorLocation` self))) (.scale (`KismetMathLibrary.Conv_VectorToTransform` (`self.K2_GetActorLocation` self)))) true))
    (if (not (`VictoryCore.IsShipping`))
      (if (`VictoryCore.IsPlayInEditor`)
        (bind _asprimaldinocharacter (cast `PrimalDinoCharacter` _returnvalue))
        (`PrimalDinoCharacter.BPUnstasis` _asprimaldinocharacter)))
    (else
      (`self.K2_DestroyActor` _returnvalue))))

(fn `UserConstructionScript`
  (`parent.UserConstructionScript`))