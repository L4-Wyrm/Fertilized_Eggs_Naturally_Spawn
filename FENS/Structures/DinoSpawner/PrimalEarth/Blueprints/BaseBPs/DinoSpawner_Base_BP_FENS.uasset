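; Base FENS dino spawner pedestal structure that, on a looping timer, randomly spawns creatures offset from itself.
; Chance rolls pick from land or marine lists, chaining into bionic and unique spawns, once per matching actor in a GetAllActorsOfClass loop.
; GameMode INI options tune chances, radii, delay and overlap-driven pedestal hiding.
; Also destroys FENS dino characters touching its collision volumes, localizes text (English, Russian, custom) and offers a destroy-pedestal use entry.
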(event `self.ReceiveBeginPlay`
  (`|ExecutionSequence`
    (:`then_0`
      (if (not (`self.bIsPreviewStructure`))
        (`|ExecutionSequence`
          (:`then_0`
            (`KismetSystemLibrary.K2_SetTimer` null "EventInitSpawn" (`self.DelayBeforeSpawn`) true))
          (:`then_1`
            (`self.INIOptions`))
          (:`then_2`
            (`self.SetSphereRadius`))
          (:`then_3`
            (`self.SetSphereHidePedestalRadius`)))))
    (:`then_1`
      (if (not (`self.bIsCustomLocalization`))
        (`self.BPCheck Game Language`)
        (else
          (`|ExecutionSequence`
            (:`then_0`
              (`self.BPGameCheckCustomLanguage`))
            (:`then_1`
              (`self.BPCusomLanguageINIOptions`))))))))

(event `EventInitSpawn`
  (`|ExecutionSequence`
    (:`then_0`
      (if (`self.bIsVanillaSpawner`)
        (`self.SpawnRandomisedDino`)))
    (:`then_1`
      (if (`self.bIsMarineSpawner`)
        (`self.SpawnRandomisedMarineDino`)))))

(event `self.PedestalHideCollisionRadius.OnComponentBeginOverlap`
  (params (OtherActor :type "Actor Object Reference") (OtherComp :type "PrimitiveComponent Object Reference") (OtherBodyIndex :type Integer) (bFromSweep :type Boolean) (SweepResult :type "EngineTypes.HitResult Structure (by ref)"))
  (if (`self.bUsePedestalAutoHide`)
    (`KismetSystemLibrary.Delay` 0.5)
    (`|ExecutionSequence`
      (:`then_0`
        (`self.SetActorHiddenInGame` false))
      (:`then_1`
        (`SceneComponent.SetVisibility` (`self.GetAllSceneComponents`) true false)))
    (if (`self.bUsePedestalAutoHideFX`) :!label _label
      (`|ExecutionSequence`
        (:`then_0`
          (`ActorComponent.Activate` (`self.ToggleMeshFX`) false))
        (:`then_1`
          (`ActorComponent.Activate` (`self.PedestalHideSound`) false))))))

(event `self.PedestalHideCollisionRadius.OnComponentEndOverlap`
  (params (OtherActor :type "Actor Object Reference") (OtherComp :type "PrimitiveComponent Object Reference") (OtherBodyIndex :type Integer))
  (if (`self.bUsePedestalAutoHide`)
    (`KismetSystemLibrary.Delay` 0.5)
    (`|ExecutionSequence`
      (:`then_0`
        (`self.SetActorHiddenInGame` true)
        (goto _label))
      (:`then_1`
        (`SceneComponent.SetVisibility` (`self.GetAllSceneComponents`) false false)
        (goto _label)))))

(event `self.EggMaxSpawnCollisionSphere.OnComponentBeginOverlap`
  (params (OtherActor :type "Actor Object Reference") (OtherComp :type "PrimitiveComponent Object Reference") (OtherBodyIndex :type Integer) (bFromSweep :type Boolean) (SweepResult :type "EngineTypes.HitResult Structure (by ref)"))
  (if (not (`self.bIsTestSpawner`))
    (bind _asdino_character_bp_fens_c (cast `/Game/Mods/FENS/CoreBlueprints/Dino_Character_BP_FENS` OtherActor))
    (if (not (`VictoryCore.IsShipping`))
      (`/Engine/EditorBlueprintResources/StandardMacros.IsValid` _asdino_character_bp_fens_c
        (:`Is Valid`
          _)))
    (`self.K2_DestroyActor` _asdino_character_bp_fens_c :!label _label_2)
    (`self.K2_DestroyActor` (stale `self.EggUnderworldDestroyCollisionBox.OnComponentHit` _asdino_character_bp_fens_c))))

(event `self.EggUnderworldDestroyCollisionBox.OnComponentHit`
  (params (OtherActor :type "Actor Object Reference") (OtherComp :type "PrimitiveComponent Object Reference") (NormalImpulse :type "Object.Vector Structure") (Hit :type "EngineTypes.HitResult Structure (by ref)"))
  (bind _asdino_character_bp_fens_c (cast `/Game/Mods/FENS/CoreBlueprints/Dino_Character_BP_FENS` OtherActor))
  (if (`VictoryCore.IsShipping`)
    (goto _label_2)
    (else
      (`/Engine/EditorBlueprintResources/StandardMacros.IsValid` _asdino_character_bp_fens_c
        (:`Is Valid`
          (goto _label_2))))))

(fn `BPCheck Game Language`
  (bind _returnvalue (`VictoryCore.GetTwoLetterISOLanguageName`))
  (`|ExecutionSequence`
    (:`then_0`
      (set `self.PedestalOptionsString` (`KismetMathLibrary.SelectString` (`self.PedestalOptionsStringRU`) (`self.PedestalOptionsStringEN`) (`KismetStringLibrary.MatchesWildcard` _returnvalue "RU"))))
    (:`then_1`
      (set `self.DestroyPedestalString` (`KismetMathLibrary.SelectString` (`self.DestroyPedestalStringEN`) (`self.DestroyPedestalStringRU`) (`KismetStringLibrary.MatchesWildcard` _returnvalue "RU")))))
  (set `self.DescriptiveName` (`KismetMathLibrary.SelectString` (`self.DescriptiveNameStringRU`) (`self.DescriptiveNameStringEN`) (`KismetStringLibrary.MatchesWildcard` _returnvalue "RU"))))

(fn `BPCusomLanguageINIOptions`
  (`/Engine/EditorBlueprintResources/ActorMacros.SwitchNetAuthority`
    (:`DedicatedServer`
      _)
    (:`PlayerServer`
      _))
  (bind _asshootergamemode (cast `ShooterGameMode` (`GameplayStatics.GetGameMode`)))
  (`|ExecutionSequence`
    (:`then_0`
      (`ShooterGameMode.InitOptionBool` _asshootergamemode "" "FENS_CustomLocalization" "UseCustomLocalization" (`self.bIsCustomLocalization`))
      (`ShooterGameMode.InitOptionString` _asshootergamemode "" "FENSSpawner_CustomLocalization" "PedestalOptionsLocalization")
      (`ShooterGameMode.InitOptionString` _asshootergamemode "" "FENSSpawner_CustomLocalization" "DestroyPedestalLocalization"))
    (:`then_1`
      (bind _returnvalue (`ShooterGameMode.GetBoolOptionIni` _asshootergamemode "FENS_CustomLocalization" "UseCustomLocalization" false))
      (set `self.bIsCustomLocalization` _returnvalue)
      (bind _returnvalue_2 (`ShooterGameMode.GetStringOption` _asshootergamemode "FENSSpawner_CustomLocalization" "PedestalOptionsLocalization"))
      (set `self.PedestalOptionsStringCustom` _returnvalue_2)
      (bind _returnvalue_3 (`ShooterGameMode.GetStringOption` _asshootergamemode "FENSSpawner_CustomLocalization" "DestroyPedestalLocalization"))
      (set `self.DestroyPedestalStringCustom` _returnvalue_3))))

(fn `BPGameCheckCustomLanguage`
  (`|ExecutionSequence`
    (:`then_0`
      (set `self.PedestalOptionsString` (`self.PedestalOptionsStringCustom`)))
    (:`then_1`
      (set `self.DestroyPedestalString` (`self.DestroyPedestalStringCustom`)))))

(fn `BPGetMultiUseEntries`
  (params (ForPC :type "PlayerController Object Reference") (MultiUseEntries :type "Array of Actor.MultiUseEntry Structure (by ref)"))
  (returns (ReturnValue :type "Array of Actor.MultiUseEntry Structure"))
  (`KismetArrayLibrary.Array_Add` MultiUseEntries (make `Actor.MultiUseEntry` null (`self.PedestalOptionsString`) 10020 4 true))
  (`KismetArrayLibrary.Array_Append` MultiUseEntries (`|MakeArray` (make `Actor.MultiUseEntry` null (`self.DestroyPedestalString`) 10021 1 false false false false false false false false false false false false false false 0 (struct :`B` 175 :`G` 175 :`R` 175 :`A` 255) (struct :`B` 255 :`G` 255 :`R` 255 :`A` 255) 0.0 3.0 (`self.DestroySound`))))
  (return MultiUseEntries))

(fn `BPTryMultiUse`
  (params (ForPC :type "PlayerController Object Reference") (UseIndex :type Integer))
  (returns (ReturnValue :type Boolean))
  (switch `int` UseIndex
    (:`Default`
      _)
    (:`10021`
      (`GameplayStatics.ApplyDamage` self 99999.9 null (`self.Instigator`))))
  (return true))

(fn `INIOptions`
  (`/Engine/EditorBlueprintResources/ActorMacros.SwitchNetAuthority`
    (:`DedicatedServer`
      _)
    (:`PlayerServer`
      _))
  (bind _asshootergamemode (cast `ShooterGameMode` (`GameplayStatics.GetGameMode`)))
  (`|ExecutionSequence`
    (:`then_0`
      (`ShooterGameMode.InitOptionFloat` _asshootergamemode "" (`self.SpawnerSettings`) (`self.SpawningChanceString`) (`self.SpawningChance`))
      (`ShooterGameMode.InitOptionFloat` _asshootergamemode "" (`self.SpawnerSettings`) (`self.MinSpawnRadiusString`) (`self.CollisionSphereMinRadius`))
      (`ShooterGameMode.InitOptionFloat` _asshootergamemode "" (`self.SpawnerSettings`) (`self.DelayBeforeSpawnString`) (`self.DelayBeforeSpawn`))
      (`ShooterGameMode.InitOptionFloat` _asshootergamemode "" (`self.SpawnerSettings`) (`self.SpawningChanceBionicString`) (`self.SpawningChanceBionic`))
      (`ShooterGameMode.InitOptionFloat` _asshootergamemode "" (`self.SpawnerSettings`) (`self.SpawningChanceUniqueString`) (`self.SpawningChanceUnique`))
      (`ShooterGameMode.InitOptionFloat` _asshootergamemode "" (`self.SpawnerSettings`) (`self.MaxSpawnRadiusString`) (`self.CollisionSphereMaxRadius`))
      (`ShooterGameMode.InitOptionFloat` _asshootergamemode "" "FENSSpawner_Settings" "RadiusAfterPedestalHide" (`self.HidePedestalSphereMaxRadius`))
      (`ShooterGameMode.InitOptionBool` _asshootergamemode "" "FENSSpawner_Settings" "UsePedestalAutoHide" (`self.bUsePedestalAutoHide`))
      (`ShooterGameMode.InitOptionBool` _asshootergamemode "" "FENSSpawner_Settings" "UsePedestalAutoHideFX" (`self.bUsePedestalAutoHideFX`)))
    (:`then_1`
      (bind _returnvalue (`ShooterGameMode.GetFloatOptionIni` _asshootergamemode (`self.SpawnerSettings`) (`self.SpawningChanceString`)))
      (set `self.SpawningChance` _returnvalue)
      (bind _returnvalue_2 (`ShooterGameMode.GetFloatOptionIni` _asshootergamemode (`self.SpawnerSettings`) (`self.MinSpawnRadiusString`)))
      (set `self.CollisionSphereMinRadius` _returnvalue_2)
      (bind _returnvalue_3 (`ShooterGameMode.GetFloatOptionIni` _asshootergamemode (`self.SpawnerSettings`) (`self.DelayBeforeSpawnString`)))
      (set `self.DelayBeforeSpawn` _returnvalue_3)
      (bind _returnvalue_4 (`ShooterGameMode.GetFloatOptionIni` _asshootergamemode (`self.SpawnerSettings`) (`self.SpawningChanceBionicString`)))
      (set `self.SpawningChanceBionic` _returnvalue_4)
      (bind _returnvalue_5 (`ShooterGameMode.GetFloatOptionIni` _asshootergamemode (`self.SpawnerSettings`) (`self.SpawningChanceUniqueString`)))
      (set `self.SpawningChanceUnique` _returnvalue_5)
      (bind _returnvalue_6 (`ShooterGameMode.GetFloatOptionIni` _asshootergamemode (`self.SpawnerSettings`) (`self.MaxSpawnRadiusString`)))
      (set `self.CollisionSphereMaxRadius` _returnvalue_6)
      (bind _returnvalue_7 (`ShooterGameMode.GetFloatOptionIni` _asshootergamemode "FENSSpawner_Settings" "RadiusAfterPedestalHide"))
      (set `self.HidePedestalSphereMaxRadius` _returnvalue_7)
      (bind _returnvalue_8 (`ShooterGameMode.GetBoolOptionIni` _asshootergamemode "FENSSpawner_Settings" "UsePedestalAutoHide" false))
      (set `self.bUsePedestalAutoHide` _returnvalue_8)
      (bind _returnvalue_9 (`ShooterGameMode.GetBoolOptionIni` _asshootergamemode "FENSSpawner_Settings" "UsePedestalAutoHideFX" false))
      (set `self.bUsePedestalAutoHideFX` _returnvalue_9))))

(fn `SetSphereHidePedestalRadius`
  (`SphereComponent.SetSphereRadius` (`self.PedestalHideCollisionRadius`) (`self.HidePedestalSphereMaxRadius`) true))

(fn `SetSphereRadius`
  (`SphereComponent.SetSphereRadius` (`self.EggMaxSpawnCollisionSphere`) (`self.CollisionSphereMinRadius`) true))

(fn `Spawn Randomised Marine Unique Dino`
  (bind _collisionsphereminradius (`self.CollisionSphereMinRadius`))
  (bind _collisionsphereminradius_2 (`self.CollisionSphereMinRadius`))
  (bind _uniquecreaturelist (`self.UniqueCreatureList`))
  (if (<= (`KismetMathLibrary.RandomFloat`) (`self.SpawningChanceUnique`))
    (bind _outactors (`GameplayStatics.GetAllActorsOfClass` null))
    (for _array_element _outactors
      (bind _asprimaldinocharacter (cast `PrimalDinoCharacter` _array_element))
      (if (`PrimalCharacter.bIsWaterDino` _asprimaldinocharacter)
        (`KismetArrayLibrary.Array_Shuffle` _uniquecreaturelist)
        (bind _returnvalue (`|SpawnActorFromClass` (`KismetArrayLibrary.Array_Get` _uniquecreaturelist (`KismetMathLibrary.RandomIntegerInRange` 0 (`KismetArrayLibrary.Array_LastIndex` (`self.UniqueCreatureList`)))) (`KismetMathLibrary.MakeTransform` (`KismetMathLibrary.MakeVector` (+ (.x (.location (`KismetMathLibrary.Conv_VectorToTransform` (`self.K2_GetActorLocation` self)))) (`KismetMathLibrary.RandomFloatInRange` _collisionsphereminradius_2 (+ _collisionsphereminradius_2 (`self.CollisionSphereMaxRadius`)))) (+ (.y (.location (`KismetMathLibrary.Conv_VectorToTransform` (`self.K2_GetActorLocation` self)))) (`KismetMathLibrary.RandomFloatInRange` _collisionsphereminradius (+ _collisionsphereminradius (`self.CollisionSphereMaxRadius`)))) (+ (.z (.location (`KismetMathLibrary.Conv_VectorToTransform` (`self.K2_GetActorLocation` self)))) 150.0)) (.rotation (`KismetMathLibrary.Conv_VectorToTransform` (`self.K2_GetActorLocation` self))) (.scale (`KismetMathLibrary.Conv_VectorToTransform` (`self.K2_GetActorLocation` self)))) true))
        (if (not (`VictoryCore.IsShipping`))
          (if (`VictoryCore.IsPlayInEditor`)
            (bind _asprimaldinocharacter_2 (cast `PrimalDinoCharacter` _returnvalue))
            (`PrimalDinoCharacter.BPUnstasis` _asprimaldinocharacter_2)))
        (else
          (`self.K2_DestroyActor` _returnvalue))))
    (else
      (`self.K2_DestroyActor` _returnvalue))))

(fn `SpawnRandomisedBionicDino`
  (bind _collisionsphereminradius (`self.CollisionSphereMinRadius`))
  (bind _collisionsphereminradius_2 (`self.CollisionSphereMinRadius`))
  (bind _bioniccreaturelist (`self.BionicCreatureList`))
  (if (<= (`KismetMathLibrary.RandomFloat`) (`self.SpawningChanceBionic`))
    (`KismetArrayLibrary.Array_Shuffle` _bioniccreaturelist)
    (bind _returnvalue (`|SpawnActorFromClass` (`KismetArrayLibrary.Array_Get` _bioniccreaturelist (`KismetMathLibrary.RandomIntegerInRange` 0 (`KismetArrayLibrary.Array_LastIndex` (`self.BionicCreatureList`)))) (`KismetMathLibrary.MakeTransform` (`KismetMathLibrary.MakeVector` (+ (.x (.location (`KismetMathLibrary.Conv_VectorToTransform` (`self.K2_GetActorLocation` self)))) (`KismetMathLibrary.RandomFloatInRange` _collisionsphereminradius_2 (+ _collisionsphereminradius_2 (`self.CollisionSphereMaxRadius`)))) (+ (.y (.location (`KismetMathLibrary.Conv_VectorToTransform` (`self.K2_GetActorLocation` self)))) (`KismetMathLibrary.RandomFloatInRange` _collisionsphereminradius (+ _collisionsphereminradius (`self.CollisionSphereMaxRadius`)))) (+ (.z (.location (`KismetMathLibrary.Conv_VectorToTransform` (`self.K2_GetActorLocation` self)))) 150.0)) (.rotation (`KismetMathLibrary.Conv_VectorToTransform` (`self.K2_GetActorLocation` self))) (.scale (`KismetMathLibrary.Conv_VectorToTransform` (`self.K2_GetActorLocation` self)))) true))
    (if (not (`VictoryCore.IsShipping`))
      (if (`VictoryCore.IsPlayInEditor`)
        (bind _asprimaldinocharacter (cast `PrimalDinoCharacter` _returnvalue))
        (`PrimalDinoCharacter.BPUnstasis` _asprimaldinocharacter)))
    (else
      (`self.K2_DestroyActor` _returnvalue))))

(fn `SpawnRandomisedDino`
  (bind _collisionsphereminradius (`self.CollisionSphereMinRadius`))
  (bind _collisionsphereminradius_2 (`self.CollisionSphereMinRadius`))
  (bind _creaturelist (`self.CreatureList`))
  (if (<= (`KismetMathLibrary.RandomFloat`) (`self.SpawningChance`))
    (bind _outactors (`GameplayStatics.GetAllActorsOfClass` null))
    (for _array_element _outactors
      (bind _asprimaldinocharacter (cast `PrimalDinoCharacter` _array_element))
      (if (not (`PrimalCharacter.bIsWaterDino` _asprimaldinocharacter))
        (`KismetArrayLibrary.Array_Shuffle` _creaturelist)
        (bind _returnvalue (`|SpawnActorFromClass` (`KismetArrayLibrary.Array_Get` _creaturelist (`KismetMathLibrary.RandomIntegerInRange` 0 (`KismetArrayLibrary.Array_LastIndex` (`self.CreatureList`)))) (`KismetMathLibrary.MakeTransform` (`KismetMathLibrary.MakeVector` (+ (.x (.location (`KismetMathLibrary.Conv_VectorToTransform` (`self.K2_GetActorLocation` self)))) (`KismetMathLibrary.RandomFloatInRange` _collisionsphereminradius_2 (+ _collisionsphereminradius_2 (`self.CollisionSphereMaxRadius`)))) (+ (.y (.location (`KismetMathLibrary.Conv_VectorToTransform` (`self.K2_GetActorLocation` self)))) (`KismetMathLibrary.RandomFloatInRange` _collisionsphereminradius (+ _collisionsphereminradius (`self.CollisionSphereMaxRadius`)))) (+ (.z (.location (`KismetMathLibrary.Conv_VectorToTransform` (`self.K2_GetActorLocation` self)))) 150.0)) (.rotation (`KismetMathLibrary.Conv_VectorToTransform` (`self.K2_GetActorLocation` self))) (.scale (`KismetMathLibrary.Conv_VectorToTransform` (`self.K2_GetActorLocation` self)))) true))
        (`|ExecutionSequence`
          (:`then_0`
            (if (not (`VictoryCore.IsShipping`))
              (if (`VictoryCore.IsPlayInEditor`)
                (bind _asprimaldinocharacter_2 (cast `PrimalDinoCharacter` _returnvalue))
                (`PrimalDinoCharacter.BPUnstasis` _asprimaldinocharacter_2))))
          (:`then_1`
            (if (`self.bIsBionicSpawner`)
              (`self.SpawnRandomisedBionicDino`)))
          (:`then_2`
            (`self.SpawnRandomisedUniqueDino`)))
        (else
          (`self.K2_DestroyActor` _returnvalue))))
    (else
      (`self.K2_DestroyActor` _asprimaldinocharacter))))

(fn `SpawnRandomisedMarineDino`
  (bind _collisionsphereminradius (`self.CollisionSphereMinRadius`))
  (bind _collisionsphereminradius_2 (`self.CollisionSphereMinRadius`))
  (bind _marinecreaturelist (`self.MarineCreatureList`))
  (if (<= (`KismetMathLibrary.RandomFloat`) (`self.SpawningChance`))
    (bind _outactors (`GameplayStatics.GetAllActorsOfClass` null))
    (for _array_element _outactors
      (bind _asprimaldinocharacter (cast `PrimalDinoCharacter` _array_element))
      (if (`PrimalCharacter.bIsWaterDino` _asprimaldinocharacter)
        (`KismetArrayLibrary.Array_Shuffle` _marinecreaturelist)
        (bind _returnvalue (`|SpawnActorFromClass` (`KismetArrayLibrary.Array_Get` _marinecreaturelist (`KismetMathLibrary.RandomIntegerInRange` 0 (`KismetArrayLibrary.Array_LastIndex` (`self.MarineCreatureList`)))) (`KismetMathLibrary.MakeTransform` (`KismetMathLibrary.MakeVector` (+ (.x (.location (`KismetMathLibrary.Conv_VectorToTransform` (`self.K2_GetActorLocation` self)))) (`KismetMathLibrary.RandomFloatInRange` _collisionsphereminradius_2 (+ _collisionsphereminradius_2 (`self.CollisionSphereMaxRadius`)))) (+ (.y (.location (`KismetMathLibrary.Conv_VectorToTransform` (`self.K2_GetActorLocation` self)))) (`KismetMathLibrary.RandomFloatInRange` _collisionsphereminradius (+ _collisionsphereminradius (`self.CollisionSphereMaxRadius`)))) (+ (.z (.location (`KismetMathLibrary.Conv_VectorToTransform` (`self.K2_GetActorLocation` self)))) 150.0)) (.rotation (`KismetMathLibrary.Conv_VectorToTransform` (`self.K2_GetActorLocation` self))) (.scale (`KismetMathLibrary.Conv_VectorToTransform` (`self.K2_GetActorLocation` self)))) true))
        (`|ExecutionSequence`
          (:`then_0`
            (if (not (`VictoryCore.IsShipping`))
              (if (`VictoryCore.IsPlayInEditor`)
                (bind _asprimaldinocharacter_2 (cast `PrimalDinoCharacter` _returnvalue))
                (`PrimalDinoCharacter.BPUnstasis` _asprimaldinocharacter_2))))
          (:`then_1`
            (if (`self.bIsBionicSpawner`)
              (`self.Spawn Randomised Marine Unique Dino`))))
        (else
          (`self.K2_DestroyActor` _returnvalue))))
    (else
      (`self.K2_DestroyActor` _returnvalue))))

(fn `SpawnRandomisedUniqueDino`
  (bind _collisionsphereminradius (`self.CollisionSphereMinRadius`))
  (bind _collisionsphereminradius_2 (`self.CollisionSphereMinRadius`))
  (bind _uniquecreaturelist (`self.UniqueCreatureList`))
  (if (<= (`KismetMathLibrary.RandomFloat`) (`self.SpawningChanceUnique`))
    (bind _outactors (`GameplayStatics.GetAllActorsOfClass` null))
    (for _array_element _outactors
      (bind _asprimaldinocharacter (cast `PrimalDinoCharacter` _array_element))
      (if (not (`PrimalCharacter.bIsWaterDino` _asprimaldinocharacter))
        (`KismetArrayLibrary.Array_Shuffle` _uniquecreaturelist)
        (bind _returnvalue (`|SpawnActorFromClass` (`KismetArrayLibrary.Array_Get` _uniquecreaturelist (`KismetMathLibrary.RandomIntegerInRange` 0 (`KismetArrayLibrary.Array_LastIndex` (`self.UniqueCreatureList`)))) (`KismetMathLibrary.MakeTransform` (`KismetMathLibrary.MakeVector` (+ (.x (.location (`KismetMathLibrary.Conv_VectorToTransform` (`self.K2_GetActorLocation` self)))) (`KismetMathLibrary.RandomFloatInRange` _collisionsphereminradius_2 (+ _collisionsphereminradius_2 (`self.CollisionSphereMaxRadius`)))) (+ (.y (.location (`KismetMathLibrary.Conv_VectorToTransform` (`self.K2_GetActorLocation` self)))) (`KismetMathLibrary.RandomFloatInRange` _collisionsphereminradius (+ _collisionsphereminradius (`self.CollisionSphereMaxRadius`)))) (+ (.z (.location (`KismetMathLibrary.Conv_VectorToTransform` (`self.K2_GetActorLocation` self)))) 150.0)) (.rotation (`KismetMathLibrary.Conv_VectorToTransform` (`self.K2_GetActorLocation` self))) (.scale (`KismetMathLibrary.Conv_VectorToTransform` (`self.K2_GetActorLocation` self)))) true))
        (if (not (`VictoryCore.IsShipping`))
          (if (`VictoryCore.IsPlayInEditor`)
            (bind _asprimaldinocharacter_2 (cast `PrimalDinoCharacter` _returnvalue))
            (`PrimalDinoCharacter.BPUnstasis` _asprimaldinocharacter_2)))
        (else
          (`self.K2_DestroyActor` _returnvalue))))
    (else
      (`self.K2_DestroyActor` _returnvalue))))

(fn `UserConstructionScript`
  (`parent.UserConstructionScript`))