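; Test dino spawner structure that randomly spawns creatures nearby, drawing from a full or eggs-only class array.
; A looping timer rolls SpawningChance and spawns above the actor at a random offset; a failed eggs-only roll destroys the spawner.
; In non-shipping play-in-editor, spawned dinos are unstasised and a random-delay callback restarts the spawn timer.
; EggMaxSpawnCollisionSphere destroys specific test dino classes that begin overlapping it.
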(event `self.ReceiveBeginPlay`
  (if (`self.bIsPreviewStructure`)
    _
    (else
      _))
  (if (`self.bSpawnOnlyEggs`)
    (`KismetSystemLibrary.K2_SetTimer` null "RandomisedTestDinoEggsOnly" 1.0 true)
    (else
      (`KismetSystemLibrary.K2_SetTimer` null "RandomisedTestDino" 1.0 true))))

(event `self.EggMaxSpawnCollisionSphere.OnComponentBeginOverlap`
  (params (OtherActor :type "Actor Object Reference") (OtherComp :type "PrimitiveComponent Object Reference") (OtherBodyIndex :type Integer) (bFromSweep :type Boolean) (SweepResult :type "EngineTypes.HitResult Structure (by ref)"))
  (`|ExecutionSequence`
    (:`then_0`
      (bind _asdino_character_test_bp_fens_c (cast `/Game/Mods/FENS/CoreBlueprints/Dino_Character_Test_BP_FENS` OtherActor))
      (`self.K2_DestroyActor` _asdino_character_test_bp_fens_c))
    (:`then_1`
      (bind _asallotestmap_character_bp_fens_c (cast `/Game/Mods/FENS/TestDinos/Allosaurus/AlloTestMap_Character_BP_FENS` OtherActor))
      (`self.K2_DestroyActor` (stale _asdilotestmap_character_bp_fens_c) :!label _label)
      (`self.K2_DestroyActor` _asallotestmap_character_bp_fens_c)
      (`self.K2_DestroyActor` (stale _asraptortestmap_character_bp_fens_c))
      (`self.K2_DestroyActor` (stale _asraptortestmap_character_bp_corrupt_fens_c))
      (`self.K2_DestroyActor` (stale _asspindlestestmap_character_bp_fens_c)))
    (:`then_2`
      (bind _asdilotestmap_character_bp_fens_c (cast `/Game/Mods/FENS/TestDinos/Dilo/DiloTestMap_Character_BP_FENS` OtherActor))
      (goto _label))
    (:`then_3`
      (bind _asraptortestmap_character_bp_fens_c (cast `/Game/Mods/FENS/TestDinos/Raptor/RaptorTestMap_Character_BP_FENS` OtherActor))
      (goto _label))
    (:`then_4`
      (bind _asraptortestmap_character_bp_corrupt_fens_c (cast `/Game/Mods/FENS/TestDinos/Corrupt/Raptor/RaptorTestMap_Character_BP_Corrupt_FENS` OtherActor))
      (goto _label))
    (:`then_5`
      (bind _asspindlestestmap_character_bp_fens_c (cast `/Game/Mods/FENS/TestDinos/Spindles/SpindlesTestMap_Character_BP_FENS` OtherActor))
      (goto _label))))

(fn `RandomisedTestDino`
  (bind _returnvalue (`KismetMathLibrary.RandomFloatInRange` -300.0 300.0))
  (bind _creaturestestarray (`self.CreaturesTestArray`))
  (if (<= (`KismetMathLibrary.RandomFloat`) (`self.SpawningChance`))
    (`KismetArrayLibrary.Array_Shuffle` _creaturestestarray)
    (bind _returnvalue_2 (`|SpawnActorFromClass` (`KismetArrayLibrary.Array_Get` _creaturestestarray (`KismetMathLibrary.RandomIntegerInRange` 0 (`KismetArrayLibrary.Array_LastIndex` (`self.CreaturesTestArray`)))) (`KismetMathLibrary.MakeTransform` (`KismetMathLibrary.MakeVector` (+ (.x (.location (`KismetMathLibrary.Conv_VectorToTransform` (`self.K2_GetActorLocation` self)))) _returnvalue) (+ (.y (.location (`KismetMathLibrary.Conv_VectorToTransform` (`self.K2_GetActorLocation` self)))) _returnvalue) (+ (.z (.location (`KismetMathLibrary.Conv_VectorToTransform` (`self.K2_GetActorLocation` self)))) (`KismetMathLibrary.RandomFloatInRange` 300.0 450.0))) (.rotation (`KismetMathLibrary.Conv_VectorToTransform` (`self.K2_GetActorLocation` self))) (.scale (`KismetMathLibrary.Conv_VectorToTransform` (`self.K2_GetActorLocation` self)))) true))
    (if (not (`VictoryCore.IsShipping`))
      (if (`VictoryCore.IsPlayInEditor`)
        (bind _asprimaldinocharacter (cast `PrimalDinoCharacter` _returnvalue_2))
        (`PrimalDinoCharacter.BPUnstasis` _asprimaldinocharacter)
        (`KismetSystemLibrary.K2_SetTimer` null "SpawnTestInterval" (`KismetMathLibrary.RandomFloatInRange` 0.0 (`self.SpawnCooldownTest`)))))))

(fn `RandomisedTestDinoEggsOnly`
  (bind _returnvalue (`KismetMathLibrary.RandomFloatInRange` -300.0 300.0))
  (bind _creaturestestarrayeggsonly (`self.CreaturesTestArrayEggsOnly`))
  (if (<= (`KismetMathLibrary.RandomFloat`) (`self.SpawningChance`))
    (`KismetArrayLibrary.Array_Shuffle` _creaturestestarrayeggsonly)
    (bind _returnvalue_2 (`|SpawnActorFromClass` (`KismetArrayLibrary.Array_Get` _creaturestestarrayeggsonly (`KismetMathLibrary.RandomIntegerInRange` 0 (`KismetArrayLibrary.Array_LastIndex` (`self.CreaturesTestArrayEggsOnly`)))) (`KismetMathLibrary.MakeTransform` (`KismetMathLibrary.MakeVector` (+ (.x (.location (`KismetMathLibrary.Conv_VectorToTransform` (`self.K2_GetActorLocation` self)))) _returnvalue) (+ (.y (.location (`KismetMathLibrary.Conv_VectorToTransform` (`self.K2_GetActorLocation` self)))) _returnvalue) (+ (.z (.location (`KismetMathLibrary.Conv_VectorToTransform` (`self.K2_GetActorLocation` self)))) (`KismetMathLibrary.RandomFloatInRange` 300.0 450.0))) (.rotation (`KismetMathLibrary.Conv_VectorToTransform` (`self.K2_GetActorLocation` self))) (.scale (`KismetMathLibrary.Conv_VectorToTransform` (`self.K2_GetActorLocation` self)))) true))
    (if (not (`VictoryCore.IsShipping`))
      (if (`VictoryCore.IsPlayInEditor`)
        (bind _asprimaldinocharacter (cast `PrimalDinoCharacter` _returnvalue_2))
        (`PrimalDinoCharacter.BPUnstasis` _asprimaldinocharacter)
        (`KismetSystemLibrary.K2_SetTimer` null "SpawnTestInterval" (`KismetMathLibrary.RandomFloatInRange` 0.0 (`self.SpawnCooldownTest`)))))
    (else
      (`self.K2_DestroyActor`))))

(fn `SpawnTestInterval`
  (if (`self.bSpawnOnlyEggs`)
    (`KismetSystemLibrary.K2_ClearTimer` null "RandomisedTestDinoEggsOnly")
    (`KismetSystemLibrary.K2_ClearTimer` null "SpawnTestInterval")
    (`KismetSystemLibrary.K2_SetTimer` null "RandomisedTestDinoEggsOnly" 1.0 true)
    (else
      (`KismetSystemLibrary.K2_ClearTimer` null "RandomisedTestDino")
      (`KismetSystemLibrary.K2_ClearTimer` null "SpawnTestInterval")
      (`KismetSystemLibrary.K2_SetTimer` null "RandomisedTestDino" 1.0 true))))

(fn `UserConstructionScript`
  (`parent.UserConstructionScript`))