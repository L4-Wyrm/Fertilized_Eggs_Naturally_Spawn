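; Inventory item for the FENS Dino Spawner structure that localizes its displayed name and description.
; On pre-initialize, it registers and reads game-mode INI options for a custom-localization toggle and custom strings.
; Name and description overrides return the custom string when enabled, otherwise Russian text for RU culture or the incoming default.
; The name lookup reuses the Russian description string rather than a separate Russian name.
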(event `self.BPPreInitializeItem`
  (params (OptionalInitWorld :type "World Object Reference"))
  (`self.BPCustomLanguageINIOptions`))

(fn `BPCheckPedestalDescriptionLanguage`
  (params (InDescription :type String))
  (returns (ReturnValue :type String))
  (return (`KismetMathLibrary.SelectString` (`KismetMathLibrary.SelectString` (`self.PedestalDescriptionStringRU`) InDescription (`KismetStringLibrary.MatchesWildcard` (`VictoryCore.GetTwoLetterISOLanguageName`) "RU")) (`self.PedestalDescriptionStringCustom`) (not (`self.bIsCustomLocalization`)))))

(fn `BPCheckPedestalNameLanguage`
  (params (InDescription :type String))
  (returns (ReturnValue :type String))
  (return (`KismetMathLibrary.SelectString` (`KismetMathLibrary.SelectString` (`self.PedestalDescriptionStringRU`) InDescription (`KismetStringLibrary.MatchesWildcard` (`VictoryCore.GetTwoLetterISOLanguageName`) "RU")) (`self.PedestalNameStringCustom`) (not (`self.bIsCustomLocalization`)))))

(fn `BPCustomLanguageINIOptions`
  (bind _asshootergamemode (cast `ShooterGameMode` (`GameplayStatics.GetGameMode` (`self.OwnerInventory`))))
  (`|ExecutionSequence`
    (:`then_0`
      (`ShooterGameMode.InitOptionBool` _asshootergamemode "" "FENS_CustomLocalization" "UseCustomLocalization" (`self.bIsCustomLocalization`))
      (`ShooterGameMode.InitOptionString` _asshootergamemode "" "FENSSpawner_CustomLocalization" (`self.PedestalNameLocalization`))
      (`ShooterGameMode.InitOptionString` _asshootergamemode "" "FENSSpawner_CustomLocalization" (`self.PedestalDescriptionLocalization`)))
    (:`then_1`
      (bind _returnvalue (`ShooterGameMode.GetBoolOptionIni` _asshootergamemode "FENS_CustomLocalization" "UseCustomLocalization" false))
      (set `self.bIsCustomLocalization` _returnvalue)
      (bind _returnvalue_2 (`ShooterGameMode.GetStringOption` _asshootergamemode "FENSSpawner_CustomLocalization" (`self.PedestalNameLocalization`)))
      (set `self.PedestalNameStringCustom` _returnvalue_2)
      (bind _returnvalue_3 (`ShooterGameMode.GetStringOption` _asshootergamemode "FENSSpawner_CustomLocalization" (`self.PedestalDescriptionLocalization`)))
      (set `self.PedestalDescriptionStringCustom` _returnvalue_3))))

(fn `BPGetItemDescription`
  (params (InDescription :type String) (bGetLongDescription :type Boolean) (ForPC :type "ShooterPlayerController Object Reference"))
  (returns (ReturnValue :type String))
  (bind _returnvalue (`self.BPCheckPedestalDescriptionLanguage` InDescription))
  (return _returnvalue))

(fn `BPGetItemName`
  (params (ItemNameIn :type String) (ForPC :type "ShooterPlayerController Object Reference"))
  (returns (ReturnValue :type String))
  (bind _returnvalue (`self.BPCheckPedestalNameLanguage` ItemNameIn))
  (return _returnvalue))