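; Genesis VR variant of the FENS DLC dino spawner, toggled by a server INI option.
; BeginPlay sets CreatureList to ClearVRCreatureList when IsVRSpawnerEnabled is true, otherwise to AddToVRCreatureList, then calls INIOptions.
; INIOptions registers and reads bIsVRSpawnerEnabled through ShooterGameMode on authority only.
; The INI value is read after the list is chosen, so that choice uses the flag's prior value.
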(event `self.ReceiveBeginPlay`
  (`|ExecutionSequence`
    (:`then_0`
      (if (`self.bIsVRSpawnerEnabled`)
        (set `self.CreatureList` (`self.ClearVRCreatureList`))
        (else
          (set `self.CreatureList` (`self.AddToVRCreatureList`)))))
    (:`then_1`
      (`self.INIOptions`))))

(fn `INIOptions`
  (`/Engine/EditorBlueprintResources/ActorMacros.Switch Has Authority`
    (:`Authority`
      (bind _asshootergamemode (cast `ShooterGameMode` (`GameplayStatics.GetGameMode`)))
      (`|ExecutionSequence`
        (:`then_0`
          (`ShooterGameMode.InitOptionBool` _asshootergamemode "" "FENSDLCSpawner_Settings" "bIsVRSpawnerEnabled" (`self.bIsVRSpawnerEnabled`)))
        (:`then_1`
          (bind _returnvalue (`ShooterGameMode.GetBoolOptionIni` _asshootergamemode "FENSDLCSpawner_Settings" "bIsVRSpawnerEnabled" false))
          (set `self.bIsVRSpawnerEnabled` _returnvalue))))))

(fn `UserConstructionScript`
  (`parent.UserConstructionScript`))