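; Base buff that plays a spawn-in effect on a dino, activating particles and sound while blocking its targeting and movement.
; It swaps the first two mesh material slots to a spawn material, then restores the cached originals after a delay and stops the effects.
; Afterwards, damage or looping checks for hostility toward local players or nearby dinos clear the movement tether.
; Another timer destroys the buff once the dino is tamed.
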(event `self.ReceiveBeginPlay`
  (`|ExecutionSequence`
    (:`then_0`
      (bind _asprimaldinocharacter (cast `PrimalDinoCharacter` (`self.GetInstigator`)))
      (`/Engine/EditorBlueprintResources/StandardMacros.IsValid` _asprimaldinocharacter
        (:`Is Valid`
          (set `PrimalCharacter.bPreventTargetingAndMovement` true _asprimaldinocharacter)
          (`self.SetSpawnDinoMaterials` _asprimaldinocharacter)
          (`KismetSystemLibrary.Delay` 5.5)
          (`self.Event_ResetDinoVanillaMaterial`)
          (`KismetSystemLibrary.K2_SetTimer` null "Event_RemoveIfTamed" 0.3 true)
          (add `self.OnTakeAnyDamage` _asprimaldinocharacter (delegate `OnTakeAnyDamage_Event`))
          (`KismetSystemLibrary.K2_SetTimer` null "Event_IsAggroToPlayer" 0.3 true)
          (`KismetSystemLibrary.K2_SetTimer` null "Event_IsAggroToOtherCreature" 0.3 true))))
    (:`then_1`
      (`ActorComponent.Activate` (`self.DinoSpawningFX`) false)
      (`ActorComponent.Activate` (`self.DinoSpawningFX_2`) false)
      (`ActorComponent.Activate` (`self.SoundToPlay`) false))))

(event `Event_ResetDinoVanillaMaterial`
  (`self.SetVanillaDinoMaterials` (stale `self.ReceiveBeginPlay` _asprimaldinocharacter))
  (set `PrimalCharacter.bPreventTargetingAndMovement` false (stale `self.ReceiveBeginPlay` _asprimaldinocharacter))
  (`ActorComponent.Activate` (`self.SoundToPlayAfter`) false)
  (`KismetSystemLibrary.Delay` 0.3)
  (`self.Event_DisableAllSpawnFX`))

(event `Event_RemoveIfTamed`
  (if (`PrimalCharacter.IsWildSlow` (stale `self.ReceiveBeginPlay` _asprimaldinocharacter))
    _
    (elif (`PrimalDinoCharacter.BPIsTamed` (stale `self.ReceiveBeginPlay` _asprimaldinocharacter))
      (`self.K2_DestroyActor`))))

(event `OnTakeAnyDamage_Event` :!signature `self.OnTakeAnyDamage`
  (params (Damage :type "Float (double-precision)") (DamageType :type "DamageType Object Reference") (InstigatedBy :type "Controller Object Reference") (DamageCauser :type "Actor Object Reference"))
  (`Pawn.ClearMovementTether` (stale `self.ReceiveBeginPlay` _asprimaldinocharacter)))

(event `Event_IsAggroToPlayer`
  (for _array_element (`VictoryCore.GetAllLocalPlayerCharacters`)
    (bind _asshootercharacter (cast `ShooterCharacter` _array_element))
    (if (`PrimalCharacter.IsHostileOrAggressiveTo` (stale `self.ReceiveBeginPlay` _asprimaldinocharacter) _asshootercharacter)
      (`Pawn.ClearMovementTether` (stale `self.ReceiveBeginPlay` _asprimaldinocharacter)))))

(event `Event_DisableAllSpawnFX`
  (`ActorComponent.Deactivate` (`self.DinoSpawningFX`))
  (`ActorComponent.Deactivate` (`self.DinoSpawningFX_2`))
  (`AudioComponent.Stop` (`self.SoundToPlay`))
  (`self.SetVanillaDinoMaterials` (stale `self.ReceiveBeginPlay` _asprimaldinocharacter)))

(event `Event_IsAggroToOtherCreature`
  (bind _returnvalue (`VictoryCore.ServerOctreeOverlapActorsClass` (`self.K2_GetWorld`) (`self.K2_GetActorLocation`) 1000.0 "DINOPAWNS" "/Script/ShooterGame.PrimalDinoCharacter"))
  (for _array_element _returnvalue
    (bind _asprimaldinocharacter (cast `PrimalDinoCharacter` _array_element))
    (`/Engine/EditorBlueprintResources/StandardMacros.IsValid` _asprimaldinocharacter
      (:`Is Valid`
        (if (`PrimalCharacter.IsHostileOrAggressiveTo` (stale `self.ReceiveBeginPlay` _asprimaldinocharacter) _asprimaldinocharacter)
          (`Pawn.ClearMovementTether` (stale `self.ReceiveBeginPlay` _asprimaldinocharacter)))))))

(fn `SetSpawnDinoMaterials`
  (params (PrimalDinoCharacterReference :type "PrimalDinoCharacter Object Reference"))
  (bind _dinospawnmaterial (`self.DinoSpawnMaterial`))
  (bind _mesh (`Character.Mesh` PrimalDinoCharacterReference))
  (`|ExecutionSequence`
    (:`then_0`
      (set `self.DinoVanillaMaterial` (`KismetArrayLibrary.Array_Get` (`MeshComponent.Materials` _mesh)))
      (bind _returnvalue (`PrimitiveComponent.CreateDynamicMaterialInstance` _mesh 0 _dinospawnmaterial))
      (`PrimitiveComponent.SetMaterial` _mesh 0 _returnvalue))
    (:`then_1`
      (set `self.DinoVanillaMaterial_2` (`KismetArrayLibrary.Array_Get` (`MeshComponent.Materials` _mesh) 1))
      (bind _returnvalue_2 (`PrimitiveComponent.CreateDynamicMaterialInstance` _mesh 1 _dinospawnmaterial))
      (`PrimitiveComponent.SetMaterial` _mesh 1 _returnvalue_2))))

(fn `SetVanillaDinoMaterials`
  (params (PrimalDinoCharacterReference :type "PrimalDinoCharacter Object Reference"))
  (bind _mesh (`Character.Mesh` PrimalDinoCharacterReference))
  (`|ExecutionSequence`
    (:`then_0`
      (bind _returnvalue (`PrimitiveComponent.CreateDynamicMaterialInstance` _mesh 0 (`self.DinoVanillaMaterial`)))
      (`PrimitiveComponent.SetMaterial` _mesh 0 _returnvalue))
    (:`then_1`
      (bind _returnvalue_2 (`PrimitiveComponent.CreateDynamicMaterialInstance` _mesh 1 (`self.DinoVanillaMaterial_2`)))
      (`PrimitiveComponent.SetMaterial` _mesh 1 _returnvalue_2))))

(fn `UserConstructionScript`
  (`parent.UserConstructionScript`))