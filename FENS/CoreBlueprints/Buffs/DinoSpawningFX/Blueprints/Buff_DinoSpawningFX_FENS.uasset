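; Buff that plays a spawn-in effect on the dino that owns it, freezing its targeting and movement while the effect runs.
; On BeginPlay it activates two spawning FX components and saves the first two mesh materials, replacing them with a spawn material, or a bionic variant for Tek dinos.
; After a fixed delay it restores the saved materials as new dynamic instances and re-enables targeting and movement.
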(event `self.ReceiveBeginPlay`
  (`|ExecutionSequence`
    (:`then_0`
      (bind _asprimaldinocharacter (cast `PrimalDinoCharacter` (`self.GetOwner`)))
      (`/Engine/EditorBlueprintResources/StandardMacros.IsValid` _asprimaldinocharacter
        (:`Is Valid`
          (if (`/Game/Mods/FENS/CoreBlueprints/Dino_Character_BP_FENS.bIsTekDino` (`self.BaseDinoReference`))
            (set `PrimalCharacter.bPreventTargetingAndMovement` true _asprimaldinocharacter)
            (`self.SetSpawnBionicDinoMaterials` _asprimaldinocharacter)
            (else
              (set `PrimalCharacter.bPreventTargetingAndMovement` true _asprimaldinocharacter)
              (`self.SetSpawnDinoMaterials` _asprimaldinocharacter)))
          (`KismetSystemLibrary.Delay` 5.5)
          (`self.Event_ResetDinoVanillaMaterial`))))
    (:`then_1`
      (`ActorComponent.Activate` (`self.DinoSpawningFX`) false)
      (`ActorComponent.Activate` (`self.DinoSpawningFX2`) false))))

(event `Event_ResetDinoVanillaMaterial`
  (`self.SetVanillaDinoMaterials` (stale `self.ReceiveBeginPlay` _asprimaldinocharacter))
  (set `PrimalCharacter.bPreventTargetingAndMovement` false (stale `self.ReceiveBeginPlay` _asprimaldinocharacter)))

(fn `SetSpawnBionicDinoMaterials`
  (params (PrimalDinoCharacterReference :type "PrimalDinoCharacter Object Reference"))
  (bind _mesh (`Character.Mesh` PrimalDinoCharacterReference))
  (`|ExecutionSequence`
    (:`then_0`
      (set `self.DinoVanillaMaterial_First` (`KismetArrayLibrary.Array_Get` (`MeshComponent.Materials` _mesh)))
      (bind _returnvalue (`PrimitiveComponent.CreateDynamicMaterialInstance` _mesh 0 (`self.BionicDinoSpawnMaterial`)))
      (`PrimitiveComponent.SetMaterial` _mesh 0 _returnvalue))
    (:`then_1`
      (set `self.DinoVanillaMaterial_Second` (`KismetArrayLibrary.Array_Get` (`MeshComponent.Materials` _mesh) 1))
      (bind _returnvalue_2 (`PrimitiveComponent.CreateDynamicMaterialInstance` _mesh 1 (`self.BionicDinoSpawnMaterial`)))
      (`PrimitiveComponent.SetMaterial` _mesh 1 _returnvalue_2))))

(fn `SetSpawnDinoMaterials`
  (params (PrimalDinoCharacterReference :type "PrimalDinoCharacter Object Reference"))
  (bind _mesh (`Character.Mesh` PrimalDinoCharacterReference))
  (`|ExecutionSequence`
    (:`then_0`
      (set `self.DinoVanillaMaterial_First` (`KismetArrayLibrary.Array_Get` (`MeshComponent.Materials` _mesh)))
      (bind _returnvalue (`PrimitiveComponent.CreateDynamicMaterialInstance` _mesh 0 (`self.DinoSpawnMaterial`)))
      (`PrimitiveComponent.SetMaterial` _mesh 0 _returnvalue))
    (:`then_1`
      (set `self.DinoVanillaMaterial_Second` (`KismetArrayLibrary.Array_Get` (`MeshComponent.Materials` _mesh) 1))
      (bind _returnvalue_2 (`PrimitiveComponent.CreateDynamicMaterialInstance` _mesh 1 (`self.DinoSpawnMaterial`)))
      (`PrimitiveComponent.SetMaterial` _mesh 1 _returnvalue_2))))

(fn `SetVanillaDinoMaterials`
  (params (PrimalDinoCharacterReference :type "PrimalDinoCharacter Object Reference"))
  (bind _mesh (`Character.Mesh` PrimalDinoCharacterReference))
  (`|ExecutionSequence`
    (:`then_0`
      (bind _returnvalue (`PrimitiveComponent.CreateDynamicMaterialInstance` _mesh 0 (`self.DinoVanillaMaterial_First`)))
      (`PrimitiveComponent.SetMaterial` _mesh 0 _returnvalue))
    (:`then_1`
      (bind _returnvalue_2 (`PrimitiveComponent.CreateDynamicMaterialInstance` _mesh 1 (`self.DinoVanillaMaterial_Second`)))
      (`PrimitiveComponent.SetMaterial` _mesh 1 _returnvalue_2))))

(fn `UserConstructionScript`
  (`parent.UserConstructionScript`))