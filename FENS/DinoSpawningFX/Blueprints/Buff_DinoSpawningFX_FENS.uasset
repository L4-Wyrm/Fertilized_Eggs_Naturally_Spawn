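; Spawn-effect buff that plays particles and transition materials on a newly spawned dino.
; On BeginPlay, servers briefly block the dino's targeting and movement, while clients and player hosts swap mesh materials to a transition instance, then a clear one after a delay.
; Bionic dinos get a separate material through per-class casts, and a timer destroys the buff.
; INIOptions can read the enable toggle from FENS_Settings, but nothing here calls it.
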(event `BlueprintTimerDynamicDelegate__DelegateSignature_Event`
  (bind _asprimaldinocharacter (cast `PrimalDinoCharacter` (`self.GetOwner`)))
  (set `PrimalCharacter.bPreventTargetingAndMovement` false _asprimaldinocharacter)
  (set `self.bIsInTransition` false true))

(event `self.ReceiveBeginPlay`
  (if (`self.bEnableDinoSpawningFX`)
    (`|ExecutionSequence`
      (:`then_0`
        (if (`self.bEnableMaterialFXOnSpawn`)
          (`|ExecutionSequence`
            (:`then_0`
              (`/Engine/EditorBlueprintResources/ActorMacros.SwitchNetAuthority`
                (:`DedicatedServer`
                  (bind _asprimaldinocharacter (cast `PrimalDinoCharacter` (`self.GetOwner`) :!label _label))
                  (set `PrimalCharacter.bPreventTargetingAndMovement` true _asprimaldinocharacter)
                  (`KismetSystemLibrary.K2_SetTimerDelegate` (delegate `BlueprintTimerDynamicDelegate__DelegateSignature_Event`) (/ 20.0 (`self.TransitionRate`)))
                  (`self.SetActorHiddenInGame` false))
                (:`PlayerServer`
                  (`|ExecutionSequence`
                    (:`then_0`
                      (bind _returnvalue (`KismetMaterialLibrary.CreateDynamicMaterialInstance` (`self.TransitionMaterial`) :!label _label_2))
                      (`/Engine/EditorBlueprintResources/StandardMacros.IsValid` _returnvalue
                        (:`Is Valid`
                          (set `self.TransitionMaterial` _returnvalue false)
                          (bind _asprimaldinocharacter_2 (cast `PrimalDinoCharacter` (`self.GetOwner`)))
                          (`|ExecutionSequence`
                            (:`then_0`
                              (bind _mesh (`Character.Mesh` _asprimaldinocharacter_2))
                              (bind _materials (`MeshComponent.Materials` _mesh))
                              (for (_array_element _array_index) _materials
                                (`/Engine/EditorBlueprintResources/StandardMacros.IsValid` _array_element
                                  (:`Is Valid`
                                    (`PrimitiveComponent.SetMaterial` _mesh _array_index (`self.TransitionMaterial`))
                                    (`KismetSystemLibrary.Delay` 3.3 :!label _label_3)
                                    (`self.EventSpawnOutMaterialInit`)))))
                            (:`then_1`
                              (for (_array_element_2 _array_index_2) _materials
                                (`/Engine/EditorBlueprintResources/StandardMacros.IsValid` _array_element_2
                                  (:`Is Valid`
                                    (`PrimitiveComponent.SetMaterial` _mesh _array_index_2 (`self.TransitionMaterial`))
                                    (goto _label_3)))))))))
                    (:`then_1`
                      (goto _label))))
                (:`Client`
                  (goto _label_2))))
            (:`then_1`
              (`self.IsBionicDino`)
              (if (`self.bIsBionicDino`)
                (`self.EventSpawnOutBionicMaterialInit`)))
            (:`then_2`
              (`KismetSystemLibrary.K2_SetTimer` null "EventSelfDestroy" 60.0)))))
      (:`then_1`
        (`ActorComponent.Activate` (`self.DinoSpawningFX`) false)
        (`ActorComponent.Activate` (`self.DinoSpawningFX2`) false)))
    (else
      (`ActorComponent.Deactivate` (`self.DinoSpawningFX`))
      (`ActorComponent.Deactivate` (`self.DinoSpawningFX2`)))))

(event `EventSpawnOutMaterialInit`
  (`/Engine/EditorBlueprintResources/ActorMacros.SwitchNetAuthority`
    (:`DedicatedServer`
      (goto _label))
    (:`PlayerServer`
      (`|ExecutionSequence`
        (:`then_0`
          _)
        (:`then_1`
          (goto _label))))
    (:`Client`
      _))
  (bind _returnvalue (`KismetMaterialLibrary.CreateDynamicMaterialInstance` (`self.TransitionMaterial`)))
  (`/Engine/EditorBlueprintResources/StandardMacros.IsValid` _returnvalue
    (:`Is Valid`
      (set `self.TransitionMaterial` _returnvalue false)
      (bind _asprimaldinocharacter (cast `PrimalDinoCharacter` (`self.GetOwner`)))
      (`|ExecutionSequence`
        (:`then_0`
          (bind _mesh (`Character.Mesh` _asprimaldinocharacter))
          (bind _materials (`MeshComponent.Materials` _mesh))
          (for (_array_element _array_index) _materials
            (`/Engine/EditorBlueprintResources/StandardMacros.IsValid` _array_element
              (:`Is Valid`
                (`PrimitiveComponent.SetMaterial` _mesh _array_index (`self.ClearTransitionMaterial`))
                (`self.EventInitOutBuff` :!label _label_4)))))
        (:`then_1`
          (for (_array_element_2 _array_index_2) _materials
            (`/Engine/EditorBlueprintResources/StandardMacros.IsValid` _array_element_2
              (:`Is Valid`
                (`PrimitiveComponent.SetMaterial` _mesh _array_index_2 (`self.ClearTransitionMaterial`))
                (goto _label_4)))))))))

(event `EventInitOutBuff`
  (`/Engine/EditorBlueprintResources/ActorMacros.SwitchNetAuthority`
    (:`DedicatedServer`
      (goto _label))
    (:`PlayerServer`
      _)
    (:`Client`
      _))
  (bind _asbuff_dinospawningfx_fens_c (cast `/FENS/DinoSpawningFX/Blueprints/Buff_DinoSpawningFX_FENS` (`self.GetOwner`)))
  (`|ExecutionSequence`
    (:`then_0`
      (`ActorComponent.Activate` (`Emitter.ParticleSystemComponent` _asbuff_dinospawningfx_fens_c) false))
    (:`then_1`
      (`ActorComponent.Activate` (`/FENS/DinoSpawningFX/Blueprints/Buff_DinoSpawningFX_FENS.SoundToPlayAfter` _asbuff_dinospawningfx_fens_c) false))))

(event `EventSpawnOutBionicMaterialInit`
  (`/Engine/EditorBlueprintResources/ActorMacros.SwitchNetAuthority`
    (:`DedicatedServer`
      (goto _label))
    (:`PlayerServer`
      (`|ExecutionSequence`
        (:`then_0`
          _)
        (:`then_1`
          (goto _label))))
    (:`Client`
      _))
  (bind _returnvalue (`KismetMaterialLibrary.CreateDynamicMaterialInstance` (`self.TransitionBionicMaterial`)))
  (`/Engine/EditorBlueprintResources/StandardMacros.IsValid` _returnvalue
    (:`Is Valid`
      (set `self.TransitionBionicMaterial` _returnvalue false)
      (`self.InitBionicDinos`))))

(event `EventSelfDestroy`
  (`self.K2_DestroyActor`))

(fn `INIOptions`
  (`/Engine/EditorBlueprintResources/ActorMacros.SwitchNetAuthority`
    (:`DedicatedServer`
      _)
    (:`PlayerServer`
      _))
  (bind _asshootergamemode (cast `ShooterGameMode` (`GameplayStatics.GetGameMode`)))
  (`|ExecutionSequence`
    (:`then_0`
      (`ShooterGameMode.InitOptionBool` _asshootergamemode "" "FENS_Settings" "EnableDinoSpawingFX" (`self.bEnableDinoSpawningFX`)))
    (:`then_1`
      (bind _returnvalue (`ShooterGameMode.GetBoolOptionIni` _asshootergamemode "FENS_Settings" "EnableDinoSpawingFX" false))
      (set `self.bEnableDinoSpawningFX` _returnvalue))))

(fn `InitBionicDinos`
  (`|ExecutionSequence`
    (:`then_0`
      (bind _asbionicpara_character_bp_c (cast `/Game/PrimalEarth/Dinos/Para/BionicPara_Character_BP` (`self.GetOwner`)))
      (`|ExecutionSequence`
        (:`then_0`
          (bind _mesh (`Character.Mesh` _asbionicpara_character_bp_c))
          (bind _materials (`MeshComponent.Materials` _mesh))
          (for (_array_element _array_index) _materials
            (`/Engine/EditorBlueprintResources/StandardMacros.IsValid` _array_element
              (:`Is Valid`
                (`PrimitiveComponent.SetMaterial` _mesh _array_index (`self.TransitionBionicMaterial`))
                (`self.EventInitOutBuff` :!label _label)))))
        (:`then_1`
          (for (_array_element_2 _array_index_2) _materials
            (`/Engine/EditorBlueprintResources/StandardMacros.IsValid` _array_element_2
              (:`Is Valid`
                (`PrimitiveComponent.SetMaterial` _mesh _array_index_2 (`self.TransitionBionicMaterial`))
                (goto _label)))))))
    (:`then_1`
      (bind _asbionicquetz_character_bp_c (cast `/Game/PrimalEarth/Dinos/Quetzalcoatlus/BionicQuetz_Character_BP` (`self.GetOwner`)))
      (`|ExecutionSequence`
        (:`then_0`
          (bind _mesh_2 (`Character.Mesh` _asbionicquetz_character_bp_c))
          (bind _materials_2 (`MeshComponent.Materials` _mesh_2))
          (for (_array_element_3 _array_index_3) _materials_2
            (`/Engine/EditorBlueprintResources/StandardMacros.IsValid` _array_element_3
              (:`Is Valid`
                (`PrimitiveComponent.SetMaterial` _mesh_2 _array_index_3 (`self.TransitionBionicMaterial`))
                (goto _label)))))
        (:`then_1`
          (for (_array_element_4 _array_index_4) _materials_2
            (`/Engine/EditorBlueprintResources/StandardMacros.IsValid` _array_element_4
              (:`Is Valid`
                (`PrimitiveComponent.SetMaterial` _mesh_2 _array_index_4 (`self.TransitionBionicMaterial`))
                (goto _label)))))))
    (:`then_2`
      (bind _asbionicraptor_character_bp_c (cast `/Game/PrimalEarth/Dinos/Raptor/BionicRaptor_Character_BP` (`self.GetOwner`)))
      (`|ExecutionSequence`
        (:`then_0`
          (bind _mesh_3 (`Character.Mesh` _asbionicraptor_character_bp_c))
          (bind _materials_3 (`MeshComponent.Materials` _mesh_3))
          (for (_array_element_5 _array_index_5) _materials_3
            (`/Engine/EditorBlueprintResources/StandardMacros.IsValid` _array_element_5
              (:`Is Valid`
                (`PrimitiveComponent.SetMaterial` _mesh_3 _array_index_5 (`self.TransitionBionicMaterial`))
                (goto _label)))))
        (:`then_1`
          (for (_array_element_6 _array_index_6) _materials_3
            (`/Engine/EditorBlueprintResources/StandardMacros.IsValid` _array_element_6
              (:`Is Valid`
                (`PrimitiveComponent.SetMaterial` _mesh_3 _array_index_6 (`self.TransitionBionicMaterial`))
                (goto _label)))))))
    (:`then_3`
      (bind _asbionicrex_character_bp_c (cast `/Game/PrimalEarth/Dinos/Rex/BionicRex_Character_BP` (`self.GetOwner`)))
      (`|ExecutionSequence`
        (:`then_0`
          (bind _mesh_4 (`Character.Mesh` _asbionicrex_character_bp_c))
          (bind _materials_4 (`MeshComponent.Materials` _mesh_4))
          (for (_array_element_7 _array_index_7) _materials_4
            (`/Engine/EditorBlueprintResources/StandardMacros.IsValid` _array_element_7
              (:`Is Valid`
                (`PrimitiveComponent.SetMaterial` _mesh_4 _array_index_7 (`self.TransitionBionicMaterial`))
                (goto _label)))))
        (:`then_1`
          (for (_array_element_8 _array_index_8) _materials_4
            (`/Engine/EditorBlueprintResources/StandardMacros.IsValid` _array_element_8
              (:`Is Valid`
                (`PrimitiveComponent.SetMaterial` _mesh_4 _array_index_8 (`self.TransitionBionicMaterial`))
                (goto _label)))))))
    (:`then_4`
      (bind _asbionicstego_character_bp_c (cast `/Game/PrimalEarth/Dinos/Stego/BionicStego_Character_BP` (`self.GetOwner`)))
      (`|ExecutionSequence`
        (:`then_0`
          (bind _mesh_5 (`Character.Mesh` _asbionicstego_character_bp_c))
          (bind _materials_5 (`MeshComponent.Materials` _mesh_5))
          (for (_array_element_9 _array_index_9) _materials_5
            (`/Engine/EditorBlueprintResources/StandardMacros.IsValid` _array_element_9
              (:`Is Valid`
                (`PrimitiveComponent.SetMaterial` _mesh_5 _array_index_9 (`self.TransitionBionicMaterial`))
                (goto _label)))))
        (:`then_1`
          (for (_array_element_10 _array_index_10) _materials_5
            (`/Engine/EditorBlueprintResources/StandardMacros.IsValid` _array_element_10
              (:`Is Valid`
                (`PrimitiveComponent.SetMaterial` _mesh_5 _array_index_10 (`self.TransitionBionicMaterial`))
                (goto _label)))))))
    (:`then_5`
      (bind _asbionictrike_character_bp_c (cast `/Game/PrimalEarth/Dinos/Trike/BionicTrike_Character_BP` (`self.GetOwner`)))
      (`|ExecutionSequence`
        (:`then_0`
          (bind _mesh_6 (`Character.Mesh` _asbionictrike_character_bp_c))
          (bind _materials_6 (`MeshComponent.Materials` _mesh_6))
          (for (_array_element_11 _array_index_11) _materials_6
            (`/Engine/EditorBlueprintResources/StandardMacros.IsValid` _array_element_11
              (:`Is Valid`
                (`PrimitiveComponent.SetMaterial` _mesh_6 _array_index_11 (`self.TransitionBionicMaterial`))
                (goto _label)))))
        (:`then_1`
          (for (_array_element_12 _array_index_12) _materials_6
            (`/Engine/EditorBlueprintResources/StandardMacros.IsValid` _array_element_12
              (:`Is Valid`
                (`PrimitiveComponent.SetMaterial` _mesh_6 _array_index_12 (`self.TransitionBionicMaterial`))
                (goto _label)))))))))

(fn `IsBionicDino`
  (bind _returnvalue (`self.GetOwner`))
  (`|ExecutionSequence`
    (:`then_0`
      (cast `/Game/PrimalEarth/Dinos/Para/BionicPara_Character_BP` _returnvalue
        (:`then`
          (set `self.bIsBionicDino` true :!label _label))
        (:`CastFailed`
          (set `self.bIsBionicDino` false :!label _label_2))))
    (:`then_1`
      (cast `/Game/PrimalEarth/Dinos/Quetzalcoatlus/BionicQuetz_Character_BP` _returnvalue
        (:`then`
          (goto _label))
        (:`CastFailed`
          (goto _label_2))))
    (:`then_2`
      (cast `/Game/PrimalEarth/Dinos/Raptor/BionicRaptor_Character_BP` _returnvalue
        (:`then`
          (goto _label))
        (:`CastFailed`
          (goto _label_2))))
    (:`then_3`
      (cast `/Game/PrimalEarth/Dinos/Rex/BionicRex_Character_BP` _returnvalue
        (:`then`
          (goto _label))
        (:`CastFailed`
          (goto _label_2))))
    (:`then_4`
      (cast `/Game/PrimalEarth/Dinos/Trike/BionicTrike_Character_BP` _returnvalue
        (:`then`
          (goto _label))
        (:`CastFailed`
          (goto _label_2))))))

(fn `UserConstructionScript`
  (`parent.UserConstructionScript`))