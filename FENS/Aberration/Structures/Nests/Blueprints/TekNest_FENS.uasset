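; TekNest_FENS is a Tek nest Blueprint from FENS that picks its mesh look and plays a spawn-in component.
; On BeginPlay it sets both material slots to either the newer ripple materials or the older nest materials, based on UseNewestTekNestMaterial.
; Only afterwards does the authority read that flag from the FENSSettings INI and initialize the option.
; After a delay, EventFinalInit activates SpawnInTek.
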(event `self.ReceiveBeginPlay`
  (bind _mystaticmesh (`self.MyStaticMesh`))
  (`parent.ReceiveBeginPlay`)
  (`|ExecutionSequence`
    (:`then_0`
      (if (`self.bUseNewestTekNestMaterial`)
        (`|ExecutionSequence`
          (:`then_0`
            (`PrimitiveComponent.SetMaterial` _mystaticmesh 0 "/Game/Mods/FENS/EndGame/Test/TekNest/MIC_TekNestRipple_FENS.MIC_TekNestRipple_FENS"))
          (:`then_1`
            (`PrimitiveComponent.SetMaterial` _mystaticmesh 1 "/Game/Mods/FENS/EndGame/Test/TekNest/MIC_TekNestSkullFeamerRipple_FENS.MIC_TekNestSkullFeamerRipple_FENS")))
        (else
          (`|ExecutionSequence`
            (:`then_0`
              (`PrimitiveComponent.SetMaterial` _mystaticmesh 0 "/Game/Aberration/Environment/DrakeTrench/Materials/Nest2_MIC.Nest2_MIC"))
            (:`then_1`
              (`PrimitiveComponent.SetMaterial` _mystaticmesh 1 "/Game/ScorchedEarth/Environment/Shared/catacomb/MI_SkullFeamer2.MI_SkullFeamer2"))))))
    (:`then_1`
      (`/Engine/EditorBlueprintResources/ActorMacros.Switch Has Authority`
        (:`Authority`
          (bind _asshootergamemode (cast `ShooterGameMode` (`GameplayStatics.GetGameMode`)))
          (bind _returnvalue (`ShooterGameMode.GetBoolOptionIni` _asshootergamemode (`self.FENS_Settings`) (`self.UseNewestNestTekMaterial`) false))
          (set `self.bUseNewestTekNestMaterial` _returnvalue)
          (`ShooterGameMode.InitOptionBool` _asshootergamemode "" (`self.FENS_Settings`) (`self.UseNewestNestTekMaterial`) (`self.bUseNewestTekNestMaterial`)))))
    (:`then_2`
      (`KismetSystemLibrary.Delay` (`self.Delay`))
      (`self.EventFinalInit`))))

(fn `EventFinalInit`
  (bind _asteknest_fens_c (cast `/FENS/Aberration/Structures/Nests/Blueprints/TekNest_FENS` self))
  (`ActorComponent.Activate` (`/FENS/Aberration/Structures/Nests/Blueprints/TekNest_FENS.SpawnInTek` _asteknest_fens_c) false))

(fn `UserConstructionScript`
  (`parent.UserConstructionScript`))